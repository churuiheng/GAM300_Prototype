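; AI-driven boat that either patrols a spline path or chases the player, using movement functions from its parent boat.
; Each living tick it throttles forward below max speed and steers by the clamped yaw toward a goal point.
; Patrol aims at the spline slightly ahead of itself; Chase aims at the first player boat when close, otherwise at the spline near that player.
; Spline goal points draw debug boxes.
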(event EventBeginPlay
  (|CallParentFunction)
  (Utilities|Array|Add (Variables|Default|GetIgnoredTargetsArray) self)
  (if (Variables|Default|GetAutoAssignTeam)
    (CallFunction|ClientAssignTeam (Variables|Default|GetTeam))))

(event Collision|EventActorBeginOverlap
  (params (OtherActor :type Actor%20Object%20Reference)))

(event EventTick
  (params (DeltaSeconds :type Float%20%28single-precision%29))
  (|CallParentFunction DeltaSeconds)
  (bind _returnvalue (Physics|GetPhysicsLinearVelocity (Variables|Default|GetBoat) "None"))
  (Variables|Default|SetisMaxSpeed (>= (Math|Vector|VectorLength _returnvalue) (Variables|Default|GetMaxSpeed)))
  (CallFunction|HandleDriftInput true true)
  (if (not (Variables|Default|GetisDead))
    (switch Utilities|FlowControl|Switch|SwitchonAIStates_Enum (Variables|Default|GetState)
      (:NewEnumerator0
        (CallFunction|HandlePatrolBehaviour))
      (:NewEnumerator1
        (CallFunction|HandleChaseBehaviour)))))

(fn ConstructionScript
  (|CallParentFunction))

(fn GetPath
  (params (Splines :type AI%20Path%20Object%20Reference))
  (bind _self self)
  (bind _path (Variables|/Game/RapidRideFightContent/Blueprints/AI_Path.AI_Path_C|GetPath Splines))
  (bind _returnvalue (Transformation|GetActorLocation _self))
  (bind _returnvalue_2 (Class|SplineComponent|FindTangentClosesttoWorldLocation _path _returnvalue "World"))
  (bind _returnvalue_3 (Math|Vector|Normalize _returnvalue_2))
  (bind _returnvalue_4 (* _returnvalue_3 5e+02))
  (bind _returnvalue_5 (+ _returnvalue_4 _returnvalue))
  (bind _returnvalue_6 (Spline|FindLocationClosesttoWorldLocation _path _returnvalue_5 "World"))
  (Rendering|Debug|DrawDebugBox :Center _returnvalue_6 :Extent "10.000000,10.000000,10.000000" :Duration 5.0)
  (return (Math|Float|MapRangeClamped (.yaw (Math|Rotator|Delta(Rotator) (Math|Rotator|FindLookatRotation _returnvalue _returnvalue_6) (Transformation|GetActorRotation))) -9e+01 9e+01 -1.0 1.0)))

(fn HandlePatrolBehaviour
  (if (Variables|Default|GetisMaxSpeed)
    _
    (else
      (CallFunction|HandleForwardMovement 1.0)))
  (bind _steeringaxis (CallFunction|GetPath (Variables|Default|GetPath)))
  (CallFunction|HandleSteering _steeringaxis))

(fn HandleChaseBehaviour
  (bind _outactors (Actor|GetAllActorsOfClass "/Game/RapidRideFightContent/Blueprints/Boat_BP_Player.Boat_BP_Player_C"))
  (if (Variables|Default|GetisMaxSpeed)
    _
    (else
      (CallFunction|HandleForwardMovement 1.0)))
  (bind _steeringaxis (CallFunction|GetPathtoTarget (Utilities|Array|Get(acopy) _outactors) (Variables|Default|GetPath)))
  (CallFunction|HandleSteering _steeringaxis))

(fn GetPathtoTarget
  (params (Target :type Boat%20BP%20Object%20Reference) (Spline :type AI%20Path%20Object%20Reference))
  (bind _returnvalue (Transformation|GetActorLocation Target))
  (bind _returnvalue_2 (Transformation|GetActorLocation Target))
  (bind _path (Variables|/Game/RapidRideFightContent/Blueprints/AI_Path.AI_Path_C|GetPath Spline))
  (bind _returnvalue_3 (Class|SplineComponent|FindTangentClosesttoWorldLocation _path _returnvalue "World"))
  (bind _returnvalue_4 (Math|Vector|Normalize _returnvalue_3))
  (bind _returnvalue_5 (* _returnvalue_4 1e+02))
  (bind _returnvalue_6 (+ _returnvalue_5 _returnvalue))
  (bind _returnvalue_7 (Spline|FindLocationClosesttoWorldLocation _path _returnvalue_6 "World"))
  (if (< (Math|Vector|Distance(Vector) _returnvalue_2 (Transformation|GetActorLocation self)) 3.2e+03)
    (return (Math|Float|MapRangeClamped (.yaw (Math|Rotator|Delta(Rotator) (Math|Rotator|FindLookatRotation (Transformation|GetActorLocation self) _returnvalue_2) (Transformation|GetActorRotation))) -9e+01 9e+01 -1.0 1.0))
    (else
      (Rendering|Debug|DrawDebugBox :Center _returnvalue_7 :Extent "10.000000,10.000000,10.000000" :Duration 5.0)
      (return (Math|Float|MapRangeClamped (.yaw (Math|Rotator|Delta(Rotator) (Math|Rotator|FindLookatRotation (Transformation|GetActorLocation self) _returnvalue_7) (Transformation|GetActorRotation))) -9e+01 9e+01 -1.0 1.0)))))