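; Boat controller for a capture-the-flag game mode that acts as the networking relay for player boat commands.
; Server events forward movement, steering, drift, boost and power use to the passed Player, triggering client boost feedback when a boost succeeds.
; It stores top and bottom HUD references through interface setters and getters.
; Pressing the 0 key starts the CTF game state's countdown.
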(event Custom|Server_HandleDrift
  (params (Player :type Boat%20BP%20Object%20Reference) (Ticks :type Float%20%28single-precision%29))
  ;[1 0.4558 0.9009] Networking: Commands to Server
  (Default|HandleDrift Player Ticks))

(event Custom|Server_UsePower
  (params (Player :type Boat%20BP%20Object%20Reference))
  ;[1 0.4558 0.9009] Networking: Commands to Server
  (Default|UsePower Player))

(event Custom|Server_HandleForwardMovement
  (params (Player :type Boat%20BP%20Player%20Object%20Reference) (Axis%20Value :type Float%20%28single-precision%29))
  ;[1 0.4558 0.9009] Networking: Commands to Server
  (Default|HandleForwardMovement Player Axis%20Value))

(event Custom|Server_HandleSteering
  (params (Player :type Boat%20BP%20Player%20Object%20Reference) (Axis%20Value :type Float%20%28single-precision%29))
  ;[1 0.4558 0.9009] Networking: Commands to Server
  (Default|HandleSteering Player Axis%20Value))

(event Custom|Server_HandleDriftInput
  (params (Player :type Boat%20BP%20Player%20Object%20Reference) (Pressed :type Boolean) (Released :type Boolean))
  ;[1 0.4558 0.9009] Networking: Commands to Server
  (Default|HandleDriftInput Player Pressed Released))

(event Custom|Server_HandleBoost
  (params (Player :type Boat%20BP%20Player%20Object%20Reference))
  ;[1 0.4558 0.9009] Networking: Commands to Server
  (bind _boostsuccess (Default|HandleBoost Player))
  (if _boostsuccess
    (Default|ClientPlayBoostFeedback Player)))

(event EventSetTopHUD
  (params (TopHUD :type W%20Top%20HUD%20Object%20Reference))
  ;[1 1 1] Interface Functions
  (Variables|Default|SetTopHUD TopHUD))

(event EventTick
  (params (DeltaSeconds :type Float%20%28single-precision%29)))

(event EventSetBottomHUD
  (params (BottomHUD :type W%20Bottom%20HUD%20UI%20Object%20Reference))
  ;[1 1 1] Interface Functions
  (Variables|Default|SetBottomHUD BottomHUD))

(event Input|KeyboardEvents|0
  (params (Key :type Key%20Structure :default "None"))
  ;[1 0.4558 0.9009] Networking: Commands to Server
  (:Pressed
    (bind _asctf_game_state_bp (Utilities|Casting|CastToCTF_GameState_BP (Game|GetGameState)))
    (Default|StartCountdown _asctf_game_state_bp)))

(fn ConstructionScript)

(fn GetBottomHUD
  (return (Variables|Default|GetBottomHUD)))

(fn GetTopHUD
  (return (Variables|Default|GetTopHUD)))