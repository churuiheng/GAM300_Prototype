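; AI patrol boat Blueprint that drives itself along a spline path using throttle, drift and steering handlers.
; Each tick while below MaxSpeed, it applies full forward input, presses drift and steers by the GetPath result.
; GetPath projects a look-ahead point along the nearest spline tangent, snaps it to the spline and maps the yaw error to clamped steering input.
; It also draws a debug box at that target point.
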(event EventBeginPlay
  (|CallParentFunction) ; This node is disabled and will not be called.\nDrag off pins to build functionality.
)

(event Collision|EventActorBeginOverlap
  (params (OtherActor :type Actor%20Object%20Reference)))

(event EventTick
  (params (DeltaSeconds :type Float%20%28single-precision%29))
  (|CallParentFunction DeltaSeconds)
  (bind _returnvalue (Physics|GetPhysicsLinearVelocity (Variables|Default|GetBoat) "None"))
  (if (< (Math|Vector|VectorLength _returnvalue) (Variables|Default|GetMaxSpeed))
    (CallFunction|HandleForwardMovement 1.0)
    (bind _steeringaxis (CallFunction|GetPath (Variables|Default|GetPath)))
    (CallFunction|HandleDriftInput true false)
    (CallFunction|HandleSteering _steeringaxis)))

(fn ConstructionScript
  (|CallParentFunction))

(fn GetPath
  (params (Splines :type AI%20Path%20Object%20Reference))
  (bind _returnvalue (Transformation|GetActorLocation))
  (bind _path (Variables|/Game/RapidRideFightContent/Blueprints/AI_Path.AI_Path_C|GetPath Splines))
  (bind _returnvalue_2 (Class|SplineComponent|FindTangentClosesttoWorldLocation _path _returnvalue "World"))
  (bind _returnvalue_3 (Math|Vector|Normalize _returnvalue_2))
  (bind _returnvalue_4 (* _returnvalue_3 5e+02))
  (bind _returnvalue_5 (+ _returnvalue_4 _returnvalue))
  (bind _returnvalue_6 (Spline|FindLocationClosesttoWorldLocation _path _returnvalue_5 "World"))
  (Rendering|Debug|DrawDebugBox :Center _returnvalue_6 :Extent "10.000000,10.000000,10.000000" :Duration 1e+01 :Thickness 4.0)
  (return (Math|Float|MapRangeClamped (.yaw (Math|Rotator|Delta(Rotator) (Math|Rotator|FindLookatRotation _returnvalue _returnvalue_6) (Transformation|GetActorRotation))) -9e+01 9e+01 -1.0 1.0)))