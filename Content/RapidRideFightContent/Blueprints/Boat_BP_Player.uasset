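; Player boat pawn that turns local input into boat driving and feeds the bottom HUD each tick with nitro and pickup updates.
; Throttle, steering, drift and boost inputs go to server handlers on the BoatController.
; A client boost event plays camera shake, force feedback and timelines animating FOV and nitrous amount.
; It also handles camera look and look-back, plus a P-key toggle that prints session ping every second.
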(event Custom|Client_PlayBoostFeedback
  ;[1 1 1] Movement
  (Camera|PlayWorldCameraShake "/Game/RapidRideFightContent/Blueprints/CameraShake_Boost.CameraShake_Boost_C" (Transformation|GetWorldLocation (Variables|Default|GetCamera)) 0.0 1e+02)
  (Game|Feedback|ClientPlayForceFeedback (Game|GetPlayerController 0) "/Game/RapidRideFightContent/ControllerFeedback/ControllerFeedback_Boost.ControllerFeedback_Boost" "None" false false false)
  (Utilities|FlowControl|Sequence
    (:then_0
      (bind _fov (Timeline|Timeline_0 PlayFromStart)
        (:Update
          (Camera|SetFieldOfView (Variables|Default|GetCamera) _fov))
        (:Finished
          (Variables|Default|SetcanBoost true)
          (Timeline|Timeline_0 SetNewTime))))
    (:then_1
      (bind _deltatime (Timeline|Timeline_1 PlayFromStart)
        (:Update
          (Variables|Default|SetNitrousAmount (+ _deltatime (Math|Conversions|ToFloat(Integer) (Variables|Default|GetNitrousCount)))))))))

(event Custom|Show%20ping
  (bind _asctf_game_instance_bp (Utilities|Casting|CastToCTF_GameInstance_BP (Game|GetGameInstance)))
  (Development|PrintString (Utilities|String|ToString(Integer) (Class|FindSessionsCallbackProxy|GetPinginMs (Variables|/Game/RapidRideFightContent/Blueprints/CTF_GameInstance_BP.CTF_GameInstance_BP_C|GetGameSession _asctf_game_instance_bp))) true true "(R=0.000000,G=0.660000,B=1.000000,A=1.000000)" 1.0))

(event EventBeginPlay
  (|CallParentFunction))

(event EventTick
  (params (DeltaSeconds :type Float%20%28single-precision%29))
  (|CallParentFunction DeltaSeconds)
  (bind _bottomhud (Class|BoatControllerBPI|GetBottomHUD(Message) (Game|GetPlayerController 0)))
  (Utilities|IsValid _bottomhud
    (:Is%20Valid
      (Default|UpdateNitroCount _bottomhud)
      (Default|UpdatePickups _bottomhud))))

(event Input|ActionEvents|InputActionDrift
  (params (Key :type Key%20Structure :default "None"))
  (bind _self self)
  (bind _boatcontroller (Variables|Default|GetBoatController))
  ;[1 1 1] Movement
  (:Pressed
    (Default|ServerHandleDriftInput _boatcontroller _self true false))
  (:Released
    (Default|ServerHandleDriftInput _boatcontroller _self false true)))

(event Input|ActionEvents|InputActionBoost
  (params (Key :type Key%20Structure :default "None"))
  ;[1 1 1] Movement
  (:Pressed
    (Default|ServerHandleBoost (Variables|Default|GetBoatController) self)))

(event Input|ActionEvents|InputActionLookBack
  (params (Key :type Key%20Structure :default "None"))
  ;[1 1 1] Look back camera
  (:Pressed
    (Transformation|AddRelativeRotation (Variables|Default|GetSpringArm) "0,180.000000, 0" false false :!label _label))
  (:Released
    (goto _label)))

(event Input|AxisEvents|InputAxisMoveForward
  (params (AxisValue :type Float%20%28single-precision%29))
  ;[1 1 1] Movement
  (Default|ServerHandleForwardMovement (Variables|Default|GetBoatController) self AxisValue))

(event Input|AxisEvents|InputAxisMoveRight
  (params (AxisValue :type Float%20%28single-precision%29))
  ;[1 1 1] Movement
  (Default|ServerHandleSteering (Variables|Default|GetBoatController) self AxisValue))

(event Input|AxisEvents|InputAxisLookUp
  (params (AxisValue :type Float%20%28single-precision%29))
  ;[1 1 1] Mouse Control
)

(event Input|AxisEvents|InputAxisTurn
  (params (AxisValue :type Float%20%28single-precision%29))
  ;[1 1 1] Mouse Control
)

(event Input|AxisEvents|InputAxisLookUpRate
  (params (AxisValue :type Float%20%28single-precision%29))
  ;[1 1 1] Mouse Control
  (Transformation|AddRelativeRotation (Variables|Default|GetCamera) (Math|Rotator|MakeRotator 0.0 AxisValue 0.0) false false))

(event Input|AxisEvents|InputAxisTurnRate
  (params (AxisValue :type Float%20%28single-precision%29))
  ;[1 1 1] Mouse Control
  (Transformation|AddRelativeRotation (Variables|Default|GetCamera) (Math|Rotator|MakeRotator 0.0 0.0 AxisValue) false false))

(event Input|KeyboardEvents|P
  (params (Key :type Key%20Structure :default "None"))
  (:Pressed
    (Utilities|FlowControl|FlipFlop
      (:A
        (bind _returnvalue (Utilities|Time|SetTimerbyEvent (delegate Custom|Show%20ping) 1.0 true))
        (Variables|Default|SetPingTimer _returnvalue))
      (:B
        (Utilities|Time|ClearandInvalidateTimerbyHandle (Variables|Default|GetPingTimer))))))

(fn ConstructionScript
  (|CallParentFunction))