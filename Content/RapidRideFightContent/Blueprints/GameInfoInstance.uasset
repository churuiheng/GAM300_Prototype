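; Game instance Blueprint that manages front-end menus and multiplayer session flow.
; Show events create main, host, server and loading screen widgets and add them to the viewport.
; Lobby launch shows the loading screen, creates a session and opens the Game level as a listen server; joining and destroying sessions are also handled.
; Session, network and travel failures route to DisplayErrorMessage, which is an empty stub, as are the error-to-string helpers.
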(event Custom|ShowMainMenu
  (bind _returnvalue (Game|GetPlayerController 0))
  ;[1 1 1] Show Main Menu
  (Utilities|IsValid (Variables|Widgets|GetMainMenuWidget)
    (:Is%20Valid
      _)
    (:Is%20Not%20Valid
      (bind _returnvalue_2 (UserInterface|CreateWidget "/Game/RapidRideFightContent/Widgets/MainMenu_WB.MainMenu_WB_C" _returnvalue))
      (Variables|Widgets|SetMainMenuWidget _returnvalue_2)))
  (UserInterface|Viewport|AddtoViewport (Variables|Widgets|GetMainMenuWidget) 0)
  (Variables|/Script/Engine.PlayerController|SetbShowMouseCursor _returnvalue true))

(event Custom|ShowHostMenu
  (bind _hostmenuwidget (Variables|Widgets|GetHostMenuWidget))
  ;[1 1 1] Show Host Menu
  (Utilities|IsValid _hostmenuwidget
    (:Is%20Valid
      _)
    (:Is%20Not%20Valid
      (UserInterface|CreateWidget "/Game/RapidRideFightContent/Widgets/HostMenu_WB.HostMenu_WB_C" (Game|GetPlayerController 0))
      (Variables|Widgets|SetMainMenuWidget _hostmenuwidget)))
  (UserInterface|Viewport|AddtoViewport _hostmenuwidget 0))

(event Custom|ShowServerMenu
  ;[1 1 1] Show Server Menu
  (bind _returnvalue (UserInterface|CreateWidget "/Game/RapidRideFightContent/Widgets/HostMenu_WB.HostMenu_WB_C" (Game|GetPlayerController 0)))
  (UserInterface|Viewport|AddtoViewport _returnvalue 0))

(event Custom|LaunchLobby
  (params (Number%20of%20Players :type Integer) (Enable%20LAN? :type Boolean) (Server%20Name :type Text))
  ;[1 1 1] Launch Lobby
  (Variables|ServerSettings|SetMaxPlayers Number%20of%20Players)
  (Variables|ServerSettings|SetServerName Server%20Name)
  (CallFunction|ShowLoadingScreen)
  (|Session (Game|GetPlayerController 0) (Variables|ServerSettings|GetMaxPlayers) Enable%20LAN?
    (:OnSuccess
      (Game|OpenLevel(byName) "Game" true "listen"))
    (:OnFailure
      (Utilities|DisplayErrorMessage "Failed to create session. Please try again."))))

(event Custom|JoinServer
  (params (SessionToJoin :type Blueprint%20Session%20Result%20Structure))
  ;[1 1 1] Join Server
  (CallFunction|ShowLoadingScreen)
  (|JoinSession (Game|GetPlayerController 0) SessionToJoin
    (:OnFailure
      (Utilities|DisplayErrorMessage "Failed to join session. Please try again."))))

(event Custom|ShowLoadingScreen
  ;[1 1 1] Show Loading Screen
  (Utilities|IsValid (Variables|Widgets|GetLoadingScreenWidget)
    (:Is%20Valid
      _)
    (:Is%20Not%20Valid
      (bind _returnvalue (UserInterface|CreateWidget "/Game/RapidRideFightContent/Widgets/LoadingScreen_WB.LoadingScreen_WB_C" (Game|GetPlayerController 0)))
      (bind _output_get (Variables|Widgets|SetLoadingScreenWidget _returnvalue))))
  (UserInterface|Viewport|AddtoViewport _output_get 0))

(event Custom|Event_NetworkError
  (params (FailureType :type ENetworkFailure%20Enum :default "NetDriverAlreadyExists") (IsServer :type Boolean))
  ;[1 1 1] Show Network Error Message
  (if IsServer
    _
    (else
      _))
  (Utilities|DisplayErrorMessage (CallFunction|NetErrortoString FailureType)))

(event Custom|Event_TravelError
  (params (FailureType :type ETravelFailure%20Enum :default "NoLevel"))
  ;[1 1 1] Show Travel Error Message
  (Utilities|DisplayErrorMessage (Utilities|String|EnumtoString FailureType)))

(event Custom|DestroySessionCaller
  (params (PlayerController :type Player%20Controller%20Object%20Reference))
  ;[1 1 1] Destroy session
  (|DestroySession PlayerController))

(fn NetErrortoString
  (params (FailureType :type ENetworkFailure%20Enum :default "NetDriverAlreadyExists"))
  (return ""))

(fn TravelErrortoString
  (params (FailureType :type ETravelFailure%20Enum :default "NoLevel"))
  (return ""))