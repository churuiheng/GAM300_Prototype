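; Behavior tree task that makes an AI boat use its nitrous boost in the boat fight game.
; It casts the controlled pawn to the AI boat and requires remaining nitrous and ability availability.
; It then triggers the boat's ability handler, plays boost feedback on success and finishes with that result, failing otherwise.
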(event EventReceiveExecuteAI
  (params (OwnerController :type AI%20Controller%20Object%20Reference) (ControlledPawn :type Pawn%20Object%20Reference))
  (bind _asboat_bp_ai (Utilities|Casting|CastToBoat_BP_AI ControlledPawn)
    (:then
      (if (and (!= (Variables|/Game/RapidRideFightContent/Blueprints/Boat_BP.Boat_BP_C|GetNitrousCount _asboat_bp_ai) 0) (Variables|/Game/RapidRideFightContent/Blueprints/Boat_BP.Boat_BP_C|GetcanUseAbility _asboat_bp_ai))
        (bind _boostsuccess (Default|HandleAbility _asboat_bp_ai))
        (if _boostsuccess
          (Default|PlayBoostFeedback _asboat_bp_ai))
        (AI|BehaviorTree|FinishExecute _boostsuccess)
        (else
          (AI|BehaviorTree|FinishExecute false))))
    (:CastFailed
      (AI|BehaviorTree|FinishExecute false))))