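; Behavior tree task that picks the next move target for an AI boat following its spline path.
; It projects a point a fixed distance ahead of the boat along the tangent of the nearest spline point, then snaps that point back onto the spline.
; The result is written to the MoveLocation blackboard key with a debug box drawn there, and the task finishes successfully.
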(event EventReceiveExecuteAI
  (params (OwnerController :type AI%20Controller%20Object%20Reference) (ControlledPawn :type Pawn%20Object%20Reference))
  (bind _asboat_bp_ai (Utilities|Casting|CastToBoat_BP_AI ControlledPawn))
  (Rendering|Debug|DrawDebugBox :Center (Spline|FindLocationClosesttoWorldLocation (Variables|/Game/RapidRideFightContent/Blueprints/AI/AI_Path.AI_Path_C|GetPath (Variables|/Game/RapidRideFightContent/Blueprints/Boat_BP_AI.Boat_BP_AI_C|GetPath _asboat_bp_ai)) (+ (* (Math|Vector|Normalize (Class|SplineComponent|FindTangentClosesttoWorldLocation (Variables|/Game/RapidRideFightContent/Blueprints/AI/AI_Path.AI_Path_C|GetPath (Variables|/Game/RapidRideFightContent/Blueprints/Boat_BP_AI.Boat_BP_AI_C|GetPath _asboat_bp_ai)) (Transformation|GetActorLocation _asboat_bp_ai) "World")) 5e+02) (Transformation|GetActorLocation _asboat_bp_ai)) "World") :Extent "10.000000,10.000000,10.000000" :Duration 1.0 :Thickness 1.0)
  (AI|BehaviorTree|SetBlackboardValueasVector (Variables|Default|GetMoveLocation) (Spline|FindLocationClosesttoWorldLocation (Variables|/Game/RapidRideFightContent/Blueprints/AI/AI_Path.AI_Path_C|GetPath (Variables|/Game/RapidRideFightContent/Blueprints/Boat_BP_AI.Boat_BP_AI_C|GetPath _asboat_bp_ai)) (+ (* (Math|Vector|Normalize (Class|SplineComponent|FindTangentClosesttoWorldLocation (Variables|/Game/RapidRideFightContent/Blueprints/AI/AI_Path.AI_Path_C|GetPath (Variables|/Game/RapidRideFightContent/Blueprints/Boat_BP_AI.Boat_BP_AI_C|GetPath _asboat_bp_ai)) (Transformation|GetActorLocation _asboat_bp_ai) "World")) 5e+02) (Transformation|GetActorLocation _asboat_bp_ai)) "World"))
  (AI|BehaviorTree|FinishExecute true))