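; Behavior tree task for the AI boat that succeeds when its seen enemy is in position to be attacked.
; It dots the enemy boat's forward vector with the direction from enemy to AI, requiring near zero, so the AI sits abeam of the enemy.
; It also requires the distance to be within AttackRange.
; A failed cast to Boat_BP_AI never finishes the task.
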(event EventReceiveExecuteAI
  (params (OwnerController :type AI%20Controller%20Object%20Reference) (ControlledPawn :type Pawn%20Object%20Reference))
  (bind _asboat_bp_ai (Utilities|Casting|CastToBoat_BP_AI ControlledPawn))
  (AI|BehaviorTree|FinishExecute (and (Math|Float|InRange(Float) (Math|Vector|DotProduct (Math|Vector|GetForwardVector (Variables|/Game/RapidRideFightContent/Blueprints/Boat_BP.Boat_BP_C|GetBoat (Variables|/Game/RapidRideFightContent/Blueprints/Boat_BP_AI.Boat_BP_AI_C|GetEnemySeen _asboat_bp_ai))) (Math|Vector|Normalize (- (Transformation|GetActorLocation _asboat_bp_ai) (Transformation|GetActorLocation (Variables|/Game/RapidRideFightContent/Blueprints/Boat_BP_AI.Boat_BP_AI_C|GetEnemySeen _asboat_bp_ai))))) -0.1 0.1) (<= (Math|Vector|VectorLength (- (Transformation|GetActorLocation _asboat_bp_ai) (Transformation|GetActorLocation (Variables|/Game/RapidRideFightContent/Blueprints/Boat_BP_AI.Boat_BP_AI_C|GetEnemySeen _asboat_bp_ai)))) (Variables|/Game/RapidRideFightContent/Blueprints/Boat_BP_AI.Boat_BP_AI_C|GetAttackRange _asboat_bp_ai)))))