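; Behavior tree task that drives an AI boat toward a target location stored in the blackboard.
; It turns on forward movement and maps the yaw difference between the boat's heading and the target direction to a clamped steering axis.
; It finishes immediately with success rather than waiting for arrival, and fails if the pawn is not a Boat_BP_AI.
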(event EventReceiveExecuteAI
  (params (OwnerController :type AI%20Controller%20Object%20Reference) (ControlledPawn :type Pawn%20Object%20Reference))
  (bind _asboat_bp_ai (Utilities|Casting|CastToBoat_BP_AI ControlledPawn)
    (:then
      (Variables|/Game/RapidRideFightContent/Blueprints/Boat_BP_AI.Boat_BP_AI_C|SetmoveForward _asboat_bp_ai true)
      (Variables|/Game/RapidRideFightContent/Blueprints/Boat_BP_AI.Boat_BP_AI_C|SetSteeringAxis _asboat_bp_ai (Math|Float|MapRangeClamped (.yaw (Math|Rotator|Delta(Rotator) (Math|Rotator|FindLookatRotation (Transformation|GetActorLocation _asboat_bp_ai) (Class|BTFunctionLibrary|GetBlackboardValueasVector (Variables|Default|GetTargetLocation))) (Transformation|GetActorRotation ControlledPawn))) -9e+01 9e+01 -1.0 1.0))
      (AI|BehaviorTree|FinishExecute true))
    (:CastFailed
      (Variables|/Game/RapidRideFightContent/Blueprints/Boat_BP_AI.Boat_BP_AI_C|SetmoveForward _asboat_bp_ai false)
      (AI|BehaviorTree|FinishExecute false))))