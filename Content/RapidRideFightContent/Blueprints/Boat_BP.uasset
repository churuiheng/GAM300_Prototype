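; Physics-driven player boat for a team capture-the-flag mode, with drifting, nitrous boosts, queued power pickups and slower speed while carrying the flag.
; Handle functions turn input into forces and rotation, while Tick adds slip-based side drag and times drifts.
; Hit-trigger overlaps on enemies report deaths to CTF_GameModeBP, unless the victim dodges within an early-drift window.
; Team assignment sets spawn, materials and HUD, and a timer refreshes flag base references.
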(event OnComponentBeginOverlap(HitTrigger)
  (params (OverlappedComponent :type Primitive%20Component%20Object%20Reference) (OtherActor :type Actor%20Object%20Reference) (OtherComp :type Primitive%20Component%20Object%20Reference) (OtherBodyIndex :type Integer) (bFromSweep :type Boolean) (SweepResult :type Hit%20Result%20Structure%20%28by%20ref%29))
  ;[1 1 1] On Boat Hit
  (if (!= (Variables|In-GameVariables|GetNitrousAmount) (Math|Conversions|ToFloat(Integer) (Variables|In-GameVariables|GetNitrousCount)))
    (bind _asboat_bp (Utilities|Casting|CastToBoat_BP OtherActor))
    (if (not (or (Variables|Boat_BP_C|GetisDead _asboat_bp) (Utilities|Enum|Equal(Enum) (Variables|Boat_BP_C|GetTeam _asboat_bp) (Variables|Parameters|GetTeam))))
      (if (and (<= (Variables|Boat_BP_C|GetDodgeWindowTime _asboat_bp) (Variables|Boat_BP_C|GetDodgeWindowDuration _asboat_bp)) (Variables|Boat_BP_C|GetisDrifting _asboat_bp))
        (CallFunction|ClientDodge _asboat_bp (Transformation|GetWorldLocation (Variables|Default|GetHitTrigger)))
        (else
          (bind _asctf_game_mode_bp (Utilities|Casting|CastToCTF_GameModeBP (Game|GetGameMode)))
          (Default|CallOnPlayerDied _asctf_game_mode_bp _asboat_bp))))))

(event Custom|Client_AssignTeam
  (params (Team :type Team_Enum%20Enum :default "NewEnumerator0"))
  ;[0.8436 0.2258 0.7316 1 48] CAPTURE THE FLAG STUFF
  ;;[0.1038 0.1038 0.1038] Assign Team
  (CallFunction|ServerAssignTeam Team)
  (CallFunction|ClientCreateHUD)
  (CallFunction|ClientSetupPlayer (Variables|Parameters|GetTeam)))

(event Custom|Server_AssignTeam
  (params (Team :type Team_Enum%20Enum :default "NewEnumerator0"))
  ;[0.8436 0.2258 0.7316 1 48] CAPTURE THE FLAG STUFF
  ;;[0.1038 0.1038 0.1038] Assign Team
  (Variables|Parameters|SetTeam Team))

(event Custom|Client_CreateHUD
  ;[0.8436 0.2258 0.7316 1 48] CAPTURE THE FLAG STUFF
  ;;[0.1038 0.1038 0.1038] Create HUD
  (bind _returnvalue (UserInterface|CreateWidget "/Game/RapidRideFightContent/Widgets_UI/HUD_WB.HUD_WB_C" (Game|GetPlayerController 0) self))
  (UserInterface|Viewport|AddtoViewport _returnvalue 0))

(event Custom|UpdateInfo
  ;[0.8436 0.2258 0.7316 1 48] CAPTURE THE FLAG STUFF
  ;;[0.1038 0.1038 0.1038] Network Update Info
  (CallFunction|ClientUpdateInfo (Variables|Parameters|GetTeam)))

(event Custom|Server_UpdateInfo
  (params (Team :type Team_Enum%20Enum :default "NewEnumerator0"))
  ;[0.8436 0.2258 0.7316 1 48] CAPTURE THE FLAG STUFF
  ;;[0.1038 0.1038 0.1038] Network Update Info
  (bind _outactors (Actor|GetAllActorsOfClass "/Game/RapidRideFightContent/Blueprints/FlagBase/FlagBase_BP.FlagBase_BP_C"))
  (bind _array_element (Utilities|Array|ForEachLoopwithBreak _outactors)
    (:LoopBody
      (if (Utilities|Enum|Equal(Enum) (Variables|/Game/RapidRideFightContent/Blueprints/FlagBase/FlagBase_BP.FlagBase_BP_C|GetTeam _array_element) Team)
        (Variables|In-GameVariables|SetMyFlagBase _array_element)
        (else
          (Variables|In-GameVariables|SetEnemyFlagBase _array_element))))))

(event Custom|Client_UpdateInfo
  (params (Team :type Team_Enum%20Enum :default "NewEnumerator0"))
  ;[0.8436 0.2258 0.7316 1 48] CAPTURE THE FLAG STUFF
  ;;[0.1038 0.1038 0.1038] Network Update Info
  (CallFunction|ServerUpdateInfo Team))

(event Custom|Client_SetupPlayer
  (params (Team :type Team_Enum%20Enum :default "NewEnumerator0"))
  (bind _returnvalue (Game|GetGameMode))
  (bind _boat (Variables|Default|GetBoat))
  (bind _flag (Variables|Default|GetFlag))
  ;[0.8436 0.2258 0.7316 1 48] CAPTURE THE FLAG STUFF
  ;;[1 1 1] Setup Player and start location
  (Utilities|IsValid _returnvalue
    (:Is%20Valid
      (bind _asctf_game_mode_bp (Utilities|Casting|CastToCTF_GameModeBP _returnvalue))
      (bind _playerstart (Default|GetPlayerStart _asctf_game_mode_bp Team))
      (Variables|Parameters|SetPlayerStart _playerstart)
      (Transformation|SetActorLocationAndRotation (.Location (Math|Transform|BreakTransform (Transformation|GetActorTransform _playerstart))) (.Rotation (Math|Transform|BreakTransform (Transformation|GetActorTransform _playerstart))))
      (Class|PrimitiveComponent|SetAllPhysicsLinearVelocity (Variables|Default|GetBoat) "0, 0, 0" false)
      (bind _asctf_game_mode_bp_2 (Utilities|Casting|CastToCTF_GameModeBP (Game|GetGameMode)))
      (if (Utilities|Enum|Equal(Enum) Team "NewEnumerator0")
        (Rendering|Material|SetMaterial _boat 0 (Variables|/Game/RapidRideFightContent/Blueprints/CTF_GameModeBP.CTF_GameModeBP_C|GetRedBoat_Material _asctf_game_mode_bp_2))
        (Rendering|Material|SetMaterial _flag 0 (Variables|/Game/RapidRideFightContent/Blueprints/CTF_GameModeBP.CTF_GameModeBP_C|GetWhiteFlag_Material _asctf_game_mode_bp_2))
        (else
          (Rendering|Material|SetMaterial _boat 0 (Variables|/Game/RapidRideFightContent/Blueprints/CTF_GameModeBP.CTF_GameModeBP_C|GetWhiteBoat_Material _asctf_game_mode_bp_2))
          (Rendering|Material|SetMaterial _flag 0 (Variables|/Game/RapidRideFightContent/Blueprints/CTF_GameModeBP.CTF_GameModeBP_C|GetRedFlag_Material _asctf_game_mode_bp_2))))
      (bind _asboat_controller_bp (Utilities|Casting|CastToBoatController_BP (Game|GetPlayerController 0)))
      (Variables|/Game/RapidRideFightContent/Blueprints/BoatController_BP.BoatController_BP_C|SetStartCountdown _asboat_controller_bp true))))

(event Custom|Client_Dodge
  (params (Hit%20Location :type Vector))
  (bind _boat (Variables|Default|GetBoat))
  (bind _returnvalue (Transformation|GetWorldRotation _boat))
  ;[1 1 1] Dodge
  (Components|Activation|Activate (Variables|Default|GetP_ElectricSpark) true)
  (if (< (Math|Vector|DotProduct (- Hit%20Location (Transformation|GetWorldLocation _boat)) (Transformation|GetActorRightVector)) 0.0)
    (bind _deltatime (Timeline|DodgeLerp PlayFromStart)
      (:Update
        (Transformation|SetWorldRotation _boat (Math|Rotator|Lerp(Rotator) _returnvalue (Math|Rotator|CombineRotators _returnvalue "0,15.000000, 0") _deltatime) false false))
      (:Finished
        (Variables|In-GameVariables|Sethit true)))
    (else
      (Timeline|DodgeLerp ReverseFromEnd))))

(event EventBeginPlay
  ;[0.8436 0.2258 0.7316 1 48] CAPTURE THE FLAG STUFF
  ;;[0.1038 0.1038 0.1038] Network Update Info
  (Utilities|Time|SetTimerbyEvent (delegate Custom|UpdateInfo) 0.25 true))

(event EventTick
  (params (DeltaSeconds :type Float%20%28single-precision%29))
  (bind _returnvalue (Transformation|GetActorRightVector))
  (bind _boat (Variables|Default|GetBoat))
  (bind _boat_2 (Variables|Default|GetBoat))
  (bind _returnvalue_2 (Transformation|GetComponentVelocity _boat_2))
  (bind _returnvalue_3 (Math|Vector|Normalize _returnvalue_2))
  ;[1 1 1] Update Loop
  (Utilities|FlowControl|Sequence
    (:then_0
      (if (or (!= (Input|AxisValues|GetMoveRight) 0.0) (> (Input|AxisValues|GetMoveForward) 0.0))
        (Variables|In-GameVariables|SetisMoving true)
        (else
          (Variables|In-GameVariables|SetisMoving false))))
    (:then_1
      ;;[1 1 1] Turn sharper, increase side drag
      (if (not (< (Math|Float|Absolute(Float) (- (.X (Math|Vector|BreakVector (Math|Rotator|GetRotationXVector (Transformation|GetWorldRotation _boat_2)))) (.X (Math|Vector|BreakVector (Math|Rotator|GetRotationXVector (Math|Conversions|RotationFromXVector _returnvalue_3)))))) (Variables|Parameters|GetSlipperyFactor)))
        (Physics|AddForce _boat (* _returnvalue (* -1 (* (Variables|Parameters|GetHandlingAmount) (* (Math|Float|Sign(Float) (Math|Vector|DotProduct _returnvalue_3 _returnvalue)) (Math|Vector|VectorLength (Transformation|GetComponentVelocity _boat)))))) "None" false)))
    (:then_2
      (CallFunction|Drift DeltaSeconds))
    (:then_3
      (if (Variables|In-GameVariables|GetisDrifting)
        (Variables|In-GameVariables|SetDodgeWindowTime (+ DeltaSeconds (Variables|In-GameVariables|GetDodgeWindowTime)))))))

(event Input|ActionEvents|InputActionUsePower
  (params (Key :type Key%20Structure))
  (bind _pickups (Variables|In-GameVariables|GetPickups))
  ;[1 1 1] On Power Use
  (:Pressed
    (if (!= (Utilities|Array|Length _pickups) 0)
      (Default|CallOnUse (Utilities|Array|Get(acopy) _pickups) self)
      (Utilities|Array|RemoveIndex _pickups))))

(event Input|KeyboardEvents|1
  (params (Key :type Key%20Structure))
  ;[0.8436 0.2258 0.7316 1 48] CAPTURE THE FLAG STUFF
  ;;[0.1038 0.1038 0.1038] Assign Team
  (:Pressed
    (CallFunction|ClientAssignTeam "NewEnumerator0")))

(event Input|GamepadEvents|GamepadLeftShoulder
  (params (Key :type Key%20Structure))
  ;[0.8436 0.2258 0.7316 1 48] CAPTURE THE FLAG STUFF
  ;;[0.1038 0.1038 0.1038] Assign Team
  (:Pressed
    (CallFunction|ClientAssignTeam "NewEnumerator1")))

(event Input|KeyboardEvents|2
  (params (Key :type Key%20Structure))
  ;[0.8436 0.2258 0.7316 1 48] CAPTURE THE FLAG STUFF
  ;;[0.1038 0.1038 0.1038] Assign Team
  (:Pressed
    (CallFunction|ClientAssignTeam "NewEnumerator1")))

(event Input|GamepadEvents|GamepadRightShoulder
  (params (Key :type Key%20Structure))
  ;[0.8436 0.2258 0.7316 1 48] CAPTURE THE FLAG STUFF
  ;;[0.1038 0.1038 0.1038] Assign Team
  (:Pressed
    (CallFunction|ClientAssignTeam "NewEnumerator0")))

(fn ConstructionScript)

(fn Drift
  (params (Ticks :type Float%20%28single-precision%29))
  (if (Variables|In-GameVariables|GetisDrifting)
    (if (< (Variables|In-GameVariables|GetDriftTime) (Variables|Parameters|GetMaxDriftDuration))
      (if (!= (Input|AxisValues|GetMoveRight) 0.0)
        (Variables|In-GameVariables|SetDriftTime (+ (Variables|In-GameVariables|GetDriftTime) Ticks))
        (Transformation|AddRelativeRotation (Variables|Default|GetBoat) (Math|Rotator|MakeRotator 0.0 0.0 (* (+ (Input|AxisValues|GetMoveForward) 1.0) (* (Variables|Parameters|GetDriftSpeed) (Input|AxisValues|GetMoveRight)))) false false)
        (bind _returnvalue (Physics|GetPhysicsLinearVelocity (Variables|Default|GetBoat) "None"))
        ;[1 1 1] Reduce slip if forward pressed and current speed less than before drift
        (if (and (< (Math|Vector|VectorLength _returnvalue) (Variables|In-GameVariables|GetspeedBeforeDrift)) (!= (Input|AxisValues|GetMoveForward) 0.0))
          (Physics|AddForce (Variables|Default|GetBoat) (* (Transformation|GetActorRightVector) (* (Input|AxisValues|GetMoveRight) (Variables|In-GameVariables|GetcurrentMovementSpeed))) "None" true)))
      (else
        (Variables|In-GameVariables|SetcanDrift false)))
    (else
      (Variables|In-GameVariables|SetDriftTime 0.0))))

(fn OnFlagPickup
  (Rendering|SetVisibility (Variables|Default|GetFlag) true false)
  (Variables|In-GameVariables|SetcurrentMovementSpeed (* (Variables|Parameters|GetSpeedRatio_WithFlag) (Variables|Parameters|GetMovementSpeed)))
  (Variables|In-GameVariables|SetisCarryingFlag true))

(fn OnFlagRemove
  (Rendering|SetVisibility (Variables|Default|GetFlag) false false)
  (Variables|In-GameVariables|SetcurrentMovementSpeed (Variables|Parameters|GetMovementSpeed))
  (Variables|In-GameVariables|SetisCarryingFlag false))

(fn RespawnPlayer
  (bind _boat (Variables|Default|GetBoat))
  (bind _playerstart (Variables|Parameters|GetPlayerStart))
  (bind _returnvalue (Transformation|GetActorTransform _playerstart))
  (bind (_location _rotation) (Math|Transform|BreakTransform _returnvalue))
  (Utilities|IsValid _playerstart
    (:Is%20Valid
      (Transformation|SetActorLocationAndRotation _location _rotation)
      (Class|PrimitiveComponent|SetAllPhysicsLinearVelocity (Variables|Default|GetBoat) "0, 0, 0" false)
      (Variables|In-GameVariables|SetisDead false)
      (bind _asctf_game_mode_bp (Utilities|Casting|CastToCTF_GameModeBP (Game|GetGameMode)))
      (if (Utilities|Enum|Equal(Enum) (Variables|Parameters|GetTeam) "NewEnumerator0")
        (Rendering|Material|SetMaterial _boat 0 (Variables|/Game/RapidRideFightContent/Blueprints/CTF_GameModeBP.CTF_GameModeBP_C|GetRedBoat_Material _asctf_game_mode_bp))
        (else
          (Rendering|Material|SetMaterial _boat 0 (Variables|/Game/RapidRideFightContent/Blueprints/CTF_GameModeBP.CTF_GameModeBP_C|GetWhiteBoat_Material _asctf_game_mode_bp)))))))

(fn HandleForwardMovement
  (params (AxisValue :type Float%20%28single-precision%29))
  (bind _returnvalue (Physics|GetPhysicsLinearVelocity (Variables|Default|GetBoat) "None"))
  (if (< (Math|Vector|VectorLength _returnvalue) (Variables|In-GameVariables|GetcurrentMaxSpeed))
    _
    (else
      _))
  (Physics|AddForce (Variables|Default|GetBoat) (* (Transformation|GetActorForwardVector) (* AxisValue (* (Variables|In-GameVariables|GetcurrentMovementSpeed) 1e+02))) "None" false)
  (Effects|SpawnEmitterAttached "/Game/RapidRideFightContent/Particles/PS_Poof.PS_Poof" (Variables|Default|GetSplashEmitter) "None" "0, 0, 0" "0, 0, 0" "1.000000,1.000000,1.000000" "KeepRelativeOffset" true "None" (Variables|In-GameVariables|GetisMoving)))

(fn HandleSteering
  (params (AxisValue :type Float%20%28single-precision%29))
  (bind _returnvalue (Transformation|GetActorLocation))
  (bind _turnspeed (Variables|Parameters|GetTurnSpeed))
  (bind _boat (Variables|Default|GetBoat))
  (bind _outhit (Collision|LineTraceByChannel _returnvalue (- _returnvalue "0, 0,300.000000") "TraceTypeQuery1" false 0 "None"))
  (if (== (.PhysMat (Collision|BreakHitResult _outhit)) "/Game/RapidRideFightContent/Materials/Physical_Materials/PhyMat_Slope_Slippery.PhyMat_Slope_Slippery")
    (Variables|In-GameVariables|SetcurrentTurnSpeed (* 0.5 _turnspeed))
    (else
      (Variables|In-GameVariables|SetcurrentTurnSpeed _turnspeed)))
  (bind _returnvalue_2 (Physics|GetPhysicsLinearVelocity (Variables|Default|GetBoat) "None"))
  (if (>= (Math|Vector|VectorLength _returnvalue_2) 0.0)
    (Transformation|AddRelativeRotation _boat (Math|Rotator|MakeRotator 0.0 0.0 (* AxisValue (Variables|In-GameVariables|GetcurrentTurnSpeed))) false false)
    (else
      (Transformation|AddRelativeRotation _boat (Math|Rotator|MakeRotator 0.0 0.0 (* -1 (* AxisValue (Variables|In-GameVariables|GetcurrentTurnSpeed)))) false false)))
  (Physics|AddForce (Variables|Default|GetBoat) (* (Transformation|GetActorRightVector) (* 1e+01 (Math|Vector|VectorLength (Transformation|GetComponentVelocity _boat)))) "None" false)
  (Effects|SpawnEmitterAttached "/Game/RapidRideFightContent/Particles/PS_Poof.PS_Poof" (Variables|Default|GetSplashEmitter) "None" "0, 0, 0" "0, 0, 0" "1.000000,1.000000,1.000000" "KeepRelativeOffset" true "None" (Variables|In-GameVariables|GetisMoving)))

(fn HandleDriftInput
  (params (Pressed :type Boolean) (Released :type Boolean))
  (Utilities|FlowControl|Sequence
    (:then_0
      (if Pressed
        (if (Variables|In-GameVariables|GetcanDrift)
          (Variables|In-GameVariables|SetisDrifting true)
          (bind _returnvalue (Physics|GetPhysicsLinearVelocity (Variables|Default|GetBoat) "None"))
          (Variables|In-GameVariables|SetspeedBeforeDrift (Math|Vector|VectorLength _returnvalue))
          (else
            (Variables|In-GameVariables|SetisDrifting false)))))
    (:then_1
      (if Released
        (Variables|In-GameVariables|SetisDrifting false)
        (Variables|In-GameVariables|SetcanDrift true)
        (Variables|In-GameVariables|SetDodgeWindowTime 0.0)))))

(fn HandleBoost
  (bind _boat (Variables|Default|GetBoat))
  (bind _nitrouscount (Variables|In-GameVariables|GetNitrousCount))
  (if (and (Variables|In-GameVariables|GetcanBoost) (> _nitrouscount 0))
    (Math|Integer|DecrementInt _nitrouscount
      (:%20%20
        (Variables|In-GameVariables|SetcanBoost false)
        (Physics|AddImpulse _boat (* (Math|Vector|GetForwardVector (Variables|Default|GetBoat)) (Variables|Parameters|GetBoosterAmount)) "None" true)
        (Physics|AddImpulseatLocation _boat "0.000000,0.000000,-10000.000000" (Transformation|GetWorldLocation (Variables|Default|GetBoostEffectLocation)) "None")
        (return true)))
    (else
      (return false))))

(fn AssignTeam
  (params (Team :type Team_Enum%20Enum :default "NewEnumerator0"))
  (CallFunction|ClientAssignTeam Team))

(fn OnPickup
  (params (Pickup :type Pickup%20Parent%20BP%20Object%20Reference))
  (bind _aspower_pickup_bp (Utilities|Casting|CastToPowerPickup_BP Pickup)
    (:then
      (if (!= (Utilities|Array|Length (Variables|In-GameVariables|GetPickups)) (Variables|Parameters|GetMaxPickups))
        (Utilities|Array|Add (Variables|In-GameVariables|GetPickups) _aspower_pickup_bp)
        (return true)
        (else
          (return false))))
    (:CastFailed
      (return true))))