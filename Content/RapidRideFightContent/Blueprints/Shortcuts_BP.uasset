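; Shortcuts_BP is an actor that provides global keyboard shortcuts, apparently for testing.
; On BeginPlay it enables input from player controller 0.
; Key events quit the game on Escape, toggle mouse cursor visibility through a FlipFlop on C, and open either the Arena02 level or the Chinatown blockout map from number keys.
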(event EventBeginPlay
  (Input|EnableInput (Game|GetPlayerController 0)))

(event Input|KeyboardEvents|C
  (params (Key :type Key%20Structure :default "None"))
  (:Pressed
    (bind _isa (Utilities|FlowControl|FlipFlop)
      (:A
        _)
      (:B
        _))
    (Variables|/Script/Engine.PlayerController|SetbShowMouseCursor (Game|GetPlayerController 0) _isa)))

(event Input|KeyboardEvents|3
  (params (Key :type Key%20Structure :default "None"))
  (:Pressed
    (Game|OpenLevel(byObjectReference) "/Game/RapidRideFightContent/Maps/LevelArena02_RH_Clean.LevelArena02_RH_Clean")))

(event Input|KeyboardEvents|4
  (params (Key :type Key%20Structure :default "None"))
  (:Pressed
    (Game|OpenLevel(byObjectReference) "/Game/RapidRideFightContent/Maps/Map_Chinatown01_Blockout.Map_Chinatown01_Blockout")))

(event Input|KeyboardEvents|Escape
  (params (Key :type Key%20Structure :default "None"))
  (:Pressed
    (Game|QuitGame 0 "Quit" false)))

(fn ConstructionScript)