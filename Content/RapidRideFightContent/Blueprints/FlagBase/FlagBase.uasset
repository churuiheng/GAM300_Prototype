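; FlagBase is a team-owned capture-the-flag base for boats, with a flag mesh and a trigger.
; An overlapping enemy boat picks up the flag if present, while a friendly boat carrying a flag adds a team point and restores the enemy base's flag.
; Server events handle pickup, scoring and reset.
; The construction script scales the base from Radius and colors base and flag by team.
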(event OnComponentBeginOverlap(Trigger)
  (params (OverlappedComponent :type Primitive%20Component%20Object%20Reference) (OtherActor :type Actor%20Object%20Reference) (OtherComp :type Primitive%20Component%20Object%20Reference) (OtherBodyIndex :type Integer) (bFromSweep :type Boolean) (SweepResult :type Hit%20Result%20Structure%20%28by%20ref%29))
  ;[1 1 1] OnTrigger
  (bind _asboat_bp (Utilities|Casting|CastToBoat_BP OtherActor))
  (if (Utilities|Enum|Equal(Enum) (Variables|/Game/RapidRideFightContent/Blueprints/Boat_BP.Boat_BP_C|GetTeam _asboat_bp) (Variables|Default|GetTeam))
    (if (Variables|/Game/RapidRideFightContent/Blueprints/Boat_BP.Boat_BP_C|GetisCarryingFlag _asboat_bp)
      (CallFunction|ServerAddPoint)
      (CallFunction|ServerResetFlag _asboat_bp))
    (elif (Variables|Default|GethasFlag)
      (CallFunction|ServerPlayerPickupFlag _asboat_bp))))

(event Custom|Server_ResetFlag
  (params (Player :type Boat%20BP%20Object%20Reference))
  (bind _enemyflagbase (Variables|/Game/RapidRideFightContent/Blueprints/Boat_BP.Boat_BP_C|GetEnemyFlagBase Player))
  (Default|OnFlagRemove Player)
  (Variables|FlagBase_C|SethasFlag _enemyflagbase true)
  (Rendering|SetVisibility (Variables|FlagBase_C|GetFlag _enemyflagbase) true false))

(event Custom|Server_AddPoint
  (Math|Integer|IncrementInt (Variables|Default|GetTeamPoints)))

(event Custom|Server_PlayerPickupFlag
  (params (Player :type Boat%20BP%20Object%20Reference))
  (Default|OnFlagPickup Player)
  (Variables|Default|SethasFlag false)
  (Rendering|SetVisibility (Variables|Default|GetFlag) false false))

(fn ConstructionScript
  (bind _base (Variables|Default|GetBase))
  (bind _flag (Variables|Default|GetFlag))
  (Transformation|SetWorldScale3D (Variables|Default|GetBase) (Math|Conversions|ToVector(Float) (Variables|Default|GetRadius)))
  (if (Utilities|Enum|Equal(Enum) (Variables|Default|GetTeam) "NewEnumerator0")
    (Rendering|Material|SetMaterial _base 0 "/Game/RapidRideFightContent/Materials/Color_Red_Mat.Color_Red_Mat")
    (Rendering|Material|SetMaterial _flag 0 "/Game/RapidRideFightContent/Materials/Color_Red_Mat.Color_Red_Mat")
    (else
      (Rendering|Material|SetMaterial _base 0 "/Game/RapidRideFightContent/Materials/Color_mat.Color_Mat")
      (Rendering|Material|SetMaterial _flag 0 "/Game/RapidRideFightContent/Materials/Color_mat.Color_Mat"))))