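; Capture-the-flag base actor for one team, where boats steal the flag or score with a carried one.
; BeginPlay colors base and flag by team using flag materials from the game state, and construction scales the base by Radius.
; Trigger overlaps call server events: enemy boats take and hide the flag, while friendly carriers add TeamPoints and restore the enemy base's flag.
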(event OnComponentBeginOverlap(Trigger)
  (params (OverlappedComponent :type Primitive%20Component%20Object%20Reference) (OtherActor :type Actor%20Object%20Reference) (OtherComp :type Primitive%20Component%20Object%20Reference) (OtherBodyIndex :type Integer) (bFromSweep :type Boolean) (SweepResult :type Hit%20Result%20Structure%20%28by%20ref%29))
  ;[1 1 1] OnTrigger
  (bind _asboat_bp (Utilities|Casting|CastToBoat_BP OtherActor))
  (if (Utilities|Enum|Equal(Enum) (Variables|/Game/RapidRideFightContent/Blueprints/Boat_BP.Boat_BP_C|GetTeam _asboat_bp) (Variables|Default|GetTeam))
    (if (Variables|/Game/RapidRideFightContent/Blueprints/Boat_BP.Boat_BP_C|GetisCarryingFlag _asboat_bp)
      (CallFunction|ServerScore _asboat_bp))
    (elif (Variables|Default|GethasFlag)
      (CallFunction|ServerPlayerPickupFlag _asboat_bp))))

(event Custom|Server_Score
  (params (ScoringPlayer :type Boat%20BP%20Object%20Reference))
  (CallFunction|Score ScoringPlayer)
  (CallFunction|ReturnFlag (Variables|/Game/RapidRideFightContent/Blueprints/Boat_BP.Boat_BP_C|GetEnemyFlagBase ScoringPlayer)))

(event Custom|Server_PlayerPickupFlag
  (params (Player :type Boat%20BP%20Object%20Reference))
  (Default|OnFlagPickup Player)
  (Variables|Default|SethasFlag false)
  (Rendering|SetVisibility (Variables|Default|GetFlag) false false))

(event EventBeginPlay
  (bind _base (Variables|Default|GetBase))
  (bind _flag (Variables|Default|GetFlag))
  (bind _asctf_game_state_bp (Utilities|Casting|CastToCTF_GameState_BP (Game|GetGameState)))
  (if (Utilities|Enum|Equal(Enum) (Variables|Default|GetTeam) "NewEnumerator0")
    (Rendering|Material|SetMaterial _base 0 "/Game/RapidRideFightContent/Materials/Flat_Colors/Mat_Color_Red.Mat_Color_Red")
    (Rendering|Material|SetMaterial _flag 0 (Variables|/Game/RapidRideFightContent/Blueprints/CTF_GameState_BP.CTF_GameState_BP_C|GetRedFlag_Material _asctf_game_state_bp))
    (else
      (Rendering|Material|SetMaterial _base 0 "/Game/RapidRideFightContent/Materials/Flat_Colors/Mat_Color.Mat_Color")
      (Rendering|Material|SetMaterial _flag 0 (Variables|/Game/RapidRideFightContent/Blueprints/CTF_GameState_BP.CTF_GameState_BP_C|GetWhiteFlag_Material _asctf_game_state_bp)))))

(fn ConstructionScript
  (Transformation|SetWorldScale3D (Variables|Default|GetBase) (Math|Conversions|ToVector(Float) (Variables|Default|GetRadius))))

(fn Score
  (params (ScoringPlayer :type Boat%20BP%20Object%20Reference))
  (Math|Integer|IncrementInt (Variables|Default|GetTeamPoints)
    (:%20%20
      (Default|OnFlagRemove ScoringPlayer))))

(fn ReturnFlag
  (Variables|FlagBase_BP_C|SethasFlag self true)
  (Rendering|SetVisibility (Variables|Default|GetFlag) true false))