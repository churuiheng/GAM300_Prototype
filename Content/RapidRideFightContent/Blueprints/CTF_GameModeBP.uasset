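; Capture-the-flag game mode for a boat game, handling player death, team colors and spawn lookup.
; The player-died event triggers an explosion, material swap and flag removal, spawns an initialized, dropped flag pickup, then respawns the player after a delay.
; SetTeam, noted as not working, colors boat and flag by team.
; GetPlayerStart finds an untaken team start, but writes Taken back unchanged, so never reserves it.
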(event Custom|SetTeam
  (params (Team :type Team_Enum%20Enum :default "NewEnumerator0") (Player :type Boat%20BP%20Object%20Reference))
  (bind _flag (Variables|/Game/RapidRideFightContent/Blueprints/Boat_BP.Boat_BP_C|GetFlag Player))
  (bind _boat (Variables|/Game/RapidRideFightContent/Blueprints/Boat_BP.Boat_BP_C|GetBoat Player))
  ;[1 1 1] Set Team (Not working)
  (Variables|/Game/RapidRideFightContent/Blueprints/Boat_BP.Boat_BP_C|SetTeam Player Team)
  (if (Utilities|Enum|Equal(Enum) Team "NewEnumerator0")
    (Rendering|Material|SetMaterial _boat 0 "/Game/RapidRideFightContent/Materials/Flat_Colors/Mat_Color_Red.Mat_Color_Red")
    (Rendering|Material|SetMaterial _flag 0 "/Game/RapidRideFightContent/Materials/Flat_Colors/Mat_Color.Mat_Color")
    (else
      (Rendering|Material|SetMaterial _boat 0 "/Game/RapidRideFightContent/Materials/Flat_Colors/Mat_Color.Mat_Color")
      (Rendering|Material|SetMaterial _flag 0 "/Game/RapidRideFightContent/Materials/Flat_Colors/Mat_Color_Red.Mat_Color_Red"))))

(event Custom|RespawnPlayer
  (params (Player :type Boat%20BP%20Object%20Reference))
  (bind _boat (Variables|/Game/RapidRideFightContent/Blueprints/Boat_BP.Boat_BP_C|GetBoat Player))
  (Effects|SpawnEmitterAttached "/Game/RapidRideFightContent/Particles/PS_Explode.PS_Explode" _boat "None" "0, 0, 0" "0, 0, 0" "1.000000,1.000000,1.000000" "SnapToTarget")
  (Rendering|Material|SetMaterial _boat 0 "/Game/Geometry/Meshes/CubeMaterial.CubeMaterial")
  (Default|OnFlagRemove Player)
  (Variables|/Game/RapidRideFightContent/Blueprints/Boat_BP.Boat_BP_C|SetisDead Player true)
  (bind _returnvalue (Game|SpawnActorfromClass "/Game/RapidRideFightContent/Blueprints/Pickups/FlagPickup_BP.FlagPickup_BP_C" (Transformation|GetWorldTransform (Variables|/Game/RapidRideFightContent/Blueprints/Boat_BP.Boat_BP_C|GetFlag Player)) "Undefined" 0 0))
  (Default|Initialize _returnvalue (Variables|/Game/RapidRideFightContent/Blueprints/FlagBase/FlagBase_BP.FlagBase_BP_C|GetTeam (Variables|/Game/RapidRideFightContent/Blueprints/Boat_BP.Boat_BP_C|GetEnemyFlagBase Player)))
  (Default|CallOnDropEvent _returnvalue)
  (Utilities|FlowControl|Delay 5.0)
  (Default|RespawnPlayer Player))

(event EventBeginPlay
  (EventDispatchers|BindEventtoOnPlayerDied (delegate Custom|RespawnPlayer)))

(fn ConstructionScript)

(fn GetPlayerStart
  (params (Team :type Team_Enum%20Enum :default "NewEnumerator0"))
  (bind _outactors (Actor|GetAllActorsOfClass "/Game/RapidRideFightContent/Blueprints/CTFPlayerStart.CTFPlayerStart_C"))
  (bind _array_element (Utilities|Array|ForEachLoopwithBreak _outactors :!label _label)
    (:LoopBody
      (if (and (Utilities|Enum|Equal(Enum) (Variables|/Game/RapidRideFightContent/Blueprints/CTFPlayerStart.CTFPlayerStart_C|GetTeam _array_element) Team) (Math|Boolean|Equal(Boolean) (Variables|/Game/RapidRideFightContent/Blueprints/CTFPlayerStart.CTFPlayerStart_C|GetTaken _array_element) false))
        (Utilities|FlowControl|Sequence
          (:then_0
            (Variables|/Game/RapidRideFightContent/Blueprints/CTFPlayerStart.CTFPlayerStart_C|SetTaken _array_element (Variables|/Game/RapidRideFightContent/Blueprints/CTFPlayerStart.CTFPlayerStart_C|GetTaken _array_element)))
          (:then_1
            (goto _label Break))
          (:then_2
            (return _array_element)))))))