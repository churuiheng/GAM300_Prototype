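; Missile Blueprint for the White Team that damages boats on hit.
; On Hit, it casts the other actor to Boat_BP and applies DamageAmount only if that boat's Team matches the first team enum entry.
; The missile then destroys itself regardless of what it struck.
; The zero-health check leads to no action, as the explosion sound and death multicast nodes are disconnected.
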(event EventBeginPlay
  (|CallParentFunction) ; This node is disabled and will not be called.\nDrag off pins to build functionality.
)

(event Collision|EventActorBeginOverlap
  (params (OtherActor :type Actor%20Object%20Reference))
  (|CallParentFunction OtherActor) ; This node is disabled and will not be called.\nDrag off pins to build functionality.
)

(event EventTick
  (params (DeltaSeconds :type Float%20%28single-precision%29))
  (|CallParentFunction DeltaSeconds) ; This node is disabled and will not be called.\nDrag off pins to build functionality.
)

(event Collision|EventHit
  (params (MyComp :type Primitive%20Component%20Object%20Reference) (Other :type Actor%20Object%20Reference) (OtherComp :type Primitive%20Component%20Object%20Reference) (bSelfMoved :type Boolean) (HitLocation :type Vector :default "0, 0, 0") (HitNormal :type Vector :default "0, 0, 0") (NormalImpulse :type Vector :default "0, 0, 0") (Hit :type Hit%20Result%20Structure%20%28by%20ref%29))
  (Utilities|FlowControl|Sequence
    (:then_0
      (bind _asboat_bp (Utilities|Casting|CastToBoat_BP Other))
      (if (Utilities|Enum|Equal(Enum) (Variables|/Game/RapidRideFightContent/Blueprints/Boat_BP.Boat_BP_C|GetTeam _asboat_bp) "NewEnumerator0")
        (Default|TakeDamage _asboat_bp (Variables|Default|GetDamage%20Amount) _asboat_bp)
        (bind _isdestroyed (Default|IsHealth0? _asboat_bp _asboat_bp))
        (if _isdestroyed
          _)))
    (:then_1
      (Actor|DestroyActor))))

(fn ConstructionScript
  (|CallParentFunction))