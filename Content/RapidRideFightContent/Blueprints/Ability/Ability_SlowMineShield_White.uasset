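; Slow mine dropped by a team, which slows and damages an enemy player who picks it up.
; On spawn it stores its team, enables physics, stops floating, pops upward and self-destructs after a drop duration.
; The inherited pickup event triggers the slow, damage and white explosion for opposing players only.
; A red-team missile overlapping its trigger also detonates it, without slowing or damaging anyone.
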(event OnComponentBeginOverlap(Trigger)
  (params (OverlappedComponent :type Primitive%20Component%20Object%20Reference) (OtherActor :type Actor%20Object%20Reference) (OtherComp :type Primitive%20Component%20Object%20Reference) (OtherBodyIndex :type Integer) (bFromSweep :type Boolean) (SweepResult :type Hit%20Result%20Structure%20%28by%20ref%29))
  (Utilities|Casting|CastToMissle_BP_RedTeam OtherActor)
  (CallFunction|Activated))

(event Custom|Activated
  (Variables|Default|SetpickedUp? true)
  (Effects|SpawnEmitteratLocation "/Game/RapidRideFightContent/Particles/PS_MineExplode_White.PS_MineExplode_White" (Transformation|GetWorldLocation (Variables|Default|GetPickup)))
  (Utilities|FlowControl|Delay 0.2)
  (Actor|DestroyActor))

(event Custom|Slow%20Player
  (params (Player :type Boat%20BP%20Object%20Reference))
  (if (Utilities|Enum|NotEqual(Enum) (Variables|/Game/RapidRideFightContent/Blueprints/Boat_BP.Boat_BP_C|GetTeam Player) (Variables|Default|GetTeam))
    (Default|OnSlowed Player (Variables|Default|GetSlowPercent) (Variables|Default|GetSlowDuration))
    (Variables|Default|SetpickedUp? true)
    (Effects|SpawnEmitteratLocation "/Game/RapidRideFightContent/Particles/PS_MineExplode_White.PS_MineExplode_White" (Transformation|GetWorldLocation (Variables|Default|GetPickup)))
    (Default|TakeDamage Player 40 Player)
    (Utilities|FlowControl|Delay 1.0)
    (Actor|DestroyActor)
    (else
      (Variables|Default|SetpickedUp? false))))

(event Custom|OnSpawn
  (params (Team :type Team_Enum%20Enum :default "NewEnumerator0"))
  (bind _base (Variables|Default|GetBase))
  (Variables|Default|SetTeam Team)
  (Physics|SetSimulatePhysics _base true)
  (Audio|Components|Audio|Stop (Variables|Default|GetFloatingAnimation))
  (Physics|AddImpulse _base (* (Math|Vector|MakeVector 0.0 0.0 1.0) 2e+02) "None" true)
  (Utilities|FlowControl|Delay (Variables|Default|GetDropDuration))
  (Actor|DestroyActor))

(event EventBeginPlay
  (|CallParentFunction)
  (EventDispatchers|BindEventtoOnPickup (delegate Custom|Slow%20Player)))

(event EventTick
  (params (DeltaSeconds :type Float%20%28single-precision%29))
  (|CallParentFunction 0.0))

(fn ConstructionScript
  (|CallParentFunction))