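; Capture-the-flag game mode for boats that tracks Red and White rosters and picks team-specific player starts.
; UpdateTeam sorts boats into rosters and counts them; AssignPlayerTeam uses those counts to randomize player 0's team or force the other when one is full.
; GetPlayerStart returns an untaken start matching the team, but writes Taken back unchanged, never reserving it.
; BeginPlay is empty, and the graph's own assign and update calls are unwired.
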(event Custom|UpdateTeam
  (bind _outactors (Actor|GetAllActorsOfClass "/Game/RapidRideFightContent/Blueprints/Boat_BP.Boat_BP_C"))
  (for _array_element _outactors
    (if (Utilities|Enum|Equal(Enum) (Variables|/Game/RapidRideFightContent/Blueprints/Boat_BP.Boat_BP_C|GetTeam _array_element) "NewEnumerator0")
      (Utilities|Array|Add (Variables|Default|GetRedTeam) _array_element)
      (CallFunction|GetRedTeam)
      (else
        (Utilities|Array|Add (Variables|Default|GetWhiteTeam) _array_element)
        (CallFunction|GetWhiteTeam)))))

(event Custom|GetWhiteTeam
  (Variables|Default|SetCurrentWhitePlayers (Utilities|Array|Length (Variables|Default|GetWhiteTeam))))

(event Custom|AssignPlayerTeam
  (if (and (< (Variables|Default|GetCurrentRedPlayers) (Variables|Default|GetMaxRedPlayers)) (< (Variables|Default|GetCurrentWhitePlayers) (Variables|Default|GetMaxWhitePlayers)))
    (CallFunction|RandomTeam)
    (elif (>= (Variables|Default|GetCurrentRedPlayers) (Variables|Default|GetMaxRedPlayers))
      (CallFunction|PlayerbeWhite)
      (elif (>= (Variables|Default|GetCurrentWhitePlayers) (Variables|Default|GetMaxWhitePlayers))
        (CallFunction|PlayerbeRed)))))

(event Custom|RandomTeam
  (bind _asboat_bp (Utilities|Casting|CastToBoat_BP (Game|Player|GetPlayerPawn 0)))
  (Default|RandomlyAssignATeam _asboat_bp))

(event Custom|PlayerBeWhite
  (bind _asboat_bp (Utilities|Casting|CastToBoat_BP (Game|Player|GetPlayerPawn 0)))
  (Default|ServerAssignTeam _asboat_bp "NewEnumerator1"))

(event Custom|PlayerBeRed
  (bind _asboat_bp (Utilities|Casting|CastToBoat_BP (Game|Player|GetPlayerPawn 0)))
  (Default|ServerAssignTeam _asboat_bp "NewEnumerator0"))

(event Custom|GetRedTeam
  (Variables|Default|SetCurrentRedPlayers (Utilities|Array|Length (Variables|Default|GetRedTeam))))

(event EventBeginPlay)

(event EventTick
  (params (DeltaSeconds :type Float%20%28single-precision%29)))

(fn ConstructionScript)

(fn GetPlayerStart
  (params (Team :type Team_Enum%20Enum :default "NewEnumerator0"))
  (bind _outactors (Actor|GetAllActorsOfClass "/Game/RapidRideFightContent/Blueprints/CTF_PlayerStart.CTF_PlayerStart_C"))
  (bind _output_get (Variables|Default|SetAllPlayerStart _outactors))
  (bind _array_element (Utilities|Array|ForEachLoopwithBreak _output_get :!label _label)
    (:LoopBody
      (if (and (Utilities|Enum|Equal(Enum) (Variables|/Game/RapidRideFightContent/Blueprints/CTF_PlayerStart.CTF_PlayerStart_C|GetTeam _array_element) Team) (Math|Boolean|Equal(Boolean) (Variables|/Game/RapidRideFightContent/Blueprints/CTF_PlayerStart.CTF_PlayerStart_C|GetTaken _array_element) false))
        (Utilities|FlowControl|Sequence
          (:then_0
            (Variables|/Game/RapidRideFightContent/Blueprints/CTF_PlayerStart.CTF_PlayerStart_C|SetTaken _array_element (Variables|/Game/RapidRideFightContent/Blueprints/CTF_PlayerStart.CTF_PlayerStart_C|GetTaken _array_element)))
          (:then_1
            (goto _label Break))
          (:then_2
            (return _array_element)))))))