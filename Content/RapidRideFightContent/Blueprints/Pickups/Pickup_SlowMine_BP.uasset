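; Slow mine pickup that slows players from a different team.
; It binds to the parent's OnPickup event, applies the slow to an opposing player and destroys itself a second later, while same-team players leave it unconsumed.
; When spawned through OnSpawn, it stores its team, turns on physics, stops the floating animation, pops upward with an impulse and expires after a drop duration.
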(event Custom|Slow%20Player
  (params (Player :type Boat%20BP%20Object%20Reference))
  (if (Utilities|Enum|NotEqual(Enum) (Variables|/Game/RapidRideFightContent/Blueprints/Boat_BP.Boat_BP_C|GetTeam Player) (Variables|Default|GetTeam))
    (Default|OnSlowed Player (Variables|Default|GetSlowPercent) (Variables|Default|GetSlowDuration))
    (Variables|Default|SetpickedUp? true)
    (Utilities|FlowControl|Delay 1.0)
    (Actor|DestroyActor)
    (else
      (Variables|Default|SetpickedUp? false))))

(event Custom|OnSpawn
  (params (Team :type Team_Enum%20Enum :default "NewEnumerator0"))
  (bind _base (Variables|Default|GetBase))
  (Variables|Default|SetTeam Team)
  (Physics|SetSimulatePhysics _base true)
  (Audio|Components|Audio|Stop (Variables|Default|GetFloatingAnimation))
  (Physics|AddImpulse _base (* (Math|Vector|MakeVector 0.0 0.0 1.0) 2e+02) "None" true)
  (Utilities|FlowControl|Delay (Variables|Default|GetDropDuration))
  (Actor|DestroyActor))

(event EventBeginPlay
  (|CallParentFunction)
  (EventDispatchers|BindEventtoOnPickup (delegate Custom|Slow%20Player)))

(event EventTick
  (params (DeltaSeconds :type Float%20%28single-precision%29))
  (|CallParentFunction 0.0))

(fn ConstructionScript
  (|CallParentFunction))