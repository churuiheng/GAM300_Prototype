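; Capture-the-flag pickup that takes its team material from the CTF game state when initialized with its flag base.
; A player of the flag's team returns it through their own base on pickup, while any other player takes it, and the pickup is destroyed shortly after.
; When dropped, it stops floating and is launched physically in a random direction with upward lift, then returns to base after a timeout.
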(event Custom|FlagDropped
  (bind _returnvalue (Math|Random|RandomUnitVector))
  (bind _base (Variables|Default|GetBase))
  ;[1 1 1] Throw the flag in a random direction when dropped
  (Physics|SetSimulatePhysics _base true)
  (Audio|Components|Audio|Stop (Variables|Default|GetFloatingAnimation))
  (Physics|AddImpulse _base (* (Math|Vector|MakeVector (.x _returnvalue) (.y _returnvalue) 0.57735) (Variables|Default|GetDropForce)) "None" true)
  (Utilities|FlowControl|Delay (Variables|Default|GetDropDuration))
  (Default|ReturnFlag (Variables|Default|GetTeamFlagBase))
  (Actor|DestroyActor))

(event Custom|HandleFlagPickup
  (params (Player :type Boat%20BP%20Object%20Reference))
  (Variables|Default|SetpickedUp true)
  (if (Utilities|Enum|Equal(Enum) (Variables|/Game/RapidRideFightContent/Blueprints/Boat_BP.Boat_BP_C|GetTeam Player) (Variables|/Game/RapidRideFightContent/Blueprints/FlagBase/FlagBase_BP.FlagBase_BP_C|GetTeam (Variables|Default|GetTeamFlagBase)))
    (Default|ReturnFlag (Variables|/Game/RapidRideFightContent/Blueprints/Boat_BP.Boat_BP_C|GetMyFlagBase Player))
    (else
      (Default|OnFlagPickup Player)))
  (Utilities|FlowControl|Delay 0.2)
  (Actor|DestroyActor))

(event EventBeginPlay
  (|CallParentFunction)
  (EventDispatchers|BindEventtoOnDropEvent (delegate Custom|FlagDropped))
  (EventDispatchers|BindEventtoOnPickup (delegate Custom|HandleFlagPickup)))

(fn ConstructionScript
  (|CallParentFunction))

(fn Initialize
  (params (TeamFlagBase :type Flag%20Base%20BP%20Object%20Reference))
  (bind _output_get (Variables|Default|SetTeamFlagBase TeamFlagBase))
  (bind _asctf_game_state_bp (Utilities|Casting|CastToCTF_GameState_BP (Game|GetGameState)))
  (switch Utilities|FlowControl|Switch|SwitchonTeam_Enum (Variables|/Game/RapidRideFightContent/Blueprints/FlagBase/FlagBase_BP.FlagBase_BP_C|GetTeam _output_get)
    (:NewEnumerator0
      (Rendering|Material|SetMaterial (Variables|Default|GetPickup) 0 (Variables|/Game/RapidRideFightContent/Blueprints/CTF_GameState_BP.CTF_GameState_BP_C|GetRedFlag_Material _asctf_game_state_bp)))
    (:NewEnumerator1
      (Rendering|Material|SetMaterial (Variables|Default|GetPickup) 0 (Variables|/Game/RapidRideFightContent/Blueprints/CTF_GameState_BP.CTF_GameState_BP_C|GetWhiteFlag_Material _asctf_game_state_bp)))))