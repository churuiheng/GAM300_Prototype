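; Pickup Blueprint that grants a power to the player who collects it, built on a parent pickup class.
; On BeginPlay it binds to the parent's OnPickup event.
; On pickup it spawns the Power class at the player's transform with the player as owner and sets its remaining uses.
; It passes that actor and its icon to the player's inventory, storing the result in PickedUp.
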(event Custom|Add%20Power%20to%20Player%20Inventory
  (params (Player :type Boat%20BP%20Object%20Reference))
  (bind _returnvalue (Game|SpawnActorfromClass (Variables|Default|GetPower) (Transformation|GetActorTransform Player) "AlwaysSpawn" Player 0))
  (Variables|/Game/RapidRideFightContent/Blueprints/Pickups/Powers/Power_BP.Power_BP_C|SetUsesLeft _returnvalue (Variables|Default|GetNumberOfUses))
  (bind _success (Default|AddPowertoInventory Player _returnvalue (Variables|Default|GetPowerIcon)))
  (Variables|Default|SetpickedUp? _success))

(event EventBeginPlay
  (|CallParentFunction)
  (EventDispatchers|BindEventtoOnPickup (delegate Custom|Add%20Power%20to%20Player%20Inventory)))

(event EventTick
  (params (DeltaSeconds :type Float%20%28single-precision%29)))

(fn ConstructionScript
  (|CallParentFunction))