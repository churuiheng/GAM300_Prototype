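; Parent Blueprint for boat pickups that bob up and down and respawn after a cooldown.
; A timeline offsets the pickup component vertically from its initial position, starting at a random playback point on BeginPlay.
; When a Boat_BP overlaps the trigger while available, it stops the animation, hides the pickup and calls the OnPickup dispatcher.
; After the Cooldown delay, it shows the pickup, re-enables collection and resumes the animation.
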(event OnComponentBeginOverlap(Trigger)
  (params (OverlappedComponent :type Primitive%20Component%20Object%20Reference) (OtherActor :type Actor%20Object%20Reference) (OtherComp :type Primitive%20Component%20Object%20Reference) (OtherBodyIndex :type Integer) (bFromSweep :type Boolean) (SweepResult :type Hit%20Result%20Structure%20%28by%20ref%29))
  (if (Variables|Private|GethasPickup)
    (Utilities|Casting|CastToBoat_BP OtherActor)
    (Audio|Components|Audio|Stop (Variables|Default|GetFloatingAnimation))
    (Variables|Private|SethasPickup false)
    (Rendering|SetVisibility (Variables|Default|GetPickup) false false)
    (Default|CallOnPickup)
    (Utilities|FlowControl|Delay (Variables|Parameters|GetCooldown))
    (Rendering|SetVisibility (Variables|Default|GetPickup) true false)
    (Variables|Private|SethasPickup true)
    (Audio|Components|Audio|Play (Variables|Default|GetFloatingAnimation))))

(event EventBeginPlay
  (bind _floatinganimation (Variables|Default|GetFloatingAnimation))
  (Variables|Private|SetFloatOffset (.Location (Math|Transform|BreakTransform (Transformation|GetRelativeTransform (Variables|Default|GetPickup)))))
  (Components|Timeline|SetPlaybackPosition _floatinganimation (Math|Random|RandomFloatinRange 0.0 (Components|Timeline|GetTimelineLength _floatinganimation)) false true))

(fn ConstructionScript)