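; Nitrous pickup Blueprint that grants nitro to the player who collects it.
; On BeginPlay it runs the parent logic, then binds its AddNitro event to the OnPickup event.
; AddNitro increments both the player's nitrous count and nitrous amount, but only while the count is below the player's maximum.
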(event Custom|Add%20Nitro
  (params (Player :type Boat%20BP%20Object%20Reference))
  (bind _nitrouscount (Variables|/Game/RapidRideFightContent/Blueprints/Boat_BP.Boat_BP_C|GetNitrousCount Player))
  (if (< _nitrouscount (Variables|/Game/RapidRideFightContent/Blueprints/Boat_BP.Boat_BP_C|GetMaxNitrousCount Player))
    (Math|Integer|IncrementInt _nitrouscount
      (:%20%20
        (Math|Float|IncrementFloat (Variables|/Game/RapidRideFightContent/Blueprints/Boat_BP.Boat_BP_C|GetNitrousAmount Player))))))

(event EventBeginPlay
  (|CallParentFunction)
  (EventDispatchers|BindEventtoOnPickup (delegate Custom|Add%20Nitro)))

(fn ConstructionScript
  (|CallParentFunction))