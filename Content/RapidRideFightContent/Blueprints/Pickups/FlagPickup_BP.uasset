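; Capture-the-flag pickup representing a team's flag, tinted red or white from the CTF game mode's materials when initialized.
; On drop it simulates physics with a randomized upward impulse, and Tick stops physics once it falls below zero height, restoring a base offset and restarting the floating animation.
; On pickup, a same-team player returns the flag to base, any other player takes it, and the actor is destroyed.
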(event Custom|FlagDropped
  (bind _returnvalue (Math|Random|RandomUnitVector))
  (bind _base (Variables|Default|GetBase))
  ;[1 1 1] Throw the flag in a random direction when dropped
  (Physics|SetSimulatePhysics _base true)
  (Audio|Components|Audio|Stop (Variables|Default|GetFloatingAnimation))
  (Physics|AddImpulse _base (* (Math|Vector|MakeVector (.x _returnvalue) (.y _returnvalue) 0.57735) (Variables|Default|GetDropForce)) "None" true))

(event Custom|HandleFlagPickup
  (params (Player :type Boat%20BP%20Object%20Reference))
  (if (Utilities|Enum|Equal(Enum) (Variables|/Game/RapidRideFightContent/Blueprints/Boat_BP.Boat_BP_C|GetTeam Player) (Variables|Default|GetTeam))
    (Default|ReturnFlag (Variables|/Game/RapidRideFightContent/Blueprints/Boat_BP.Boat_BP_C|GetMyFlagBase Player))
    (else
      (Default|OnFlagPickup Player)))
  (Actor|DestroyActor))

(event EventBeginPlay
  (|CallParentFunction)
  (EventDispatchers|BindEventtoOnDropEvent (delegate Custom|FlagDropped))
  (EventDispatchers|BindEventtoOnPickup (delegate Custom|HandleFlagPickup)))

(event EventTick
  (params (DeltaSeconds :type Float%20%28single-precision%29))
  (bind _base (Variables|Default|GetBase))
  (bind _relativelocation (Variables|/Script/Engine.SceneComponent|GetRelativeLocation _base))
  ;[1 1 1] Drop onto ground and start floating
  (if (< (.z _relativelocation) 0.0)
    (Physics|SetSimulatePhysics (Variables|Default|GetBase) false)
    (Transformation|SetWorldLocation (Variables|Default|GetBase) (Math|Vector|MakeVector (.x _relativelocation) (.y _relativelocation) (Variables|Default|GetBaseOffset)) false false)
    (Components|Timeline|PlayfromStart (Variables|Default|GetFloatingAnimation))))

(fn ConstructionScript
  (|CallParentFunction))

(fn Initialize
  (params (Team :type Team_Enum%20Enum :default "NewEnumerator0"))
  (bind _output_get (Variables|Default|SetTeam Team))
  (bind _asctf_game_mode_bp (Utilities|Casting|CastToCTF_GameModeBP (Game|GetGameMode)))
  (switch Utilities|FlowControl|Switch|SwitchonTeam_Enum _output_get
    (:NewEnumerator0
      (Rendering|Material|SetMaterial (Variables|Default|GetPickup) 0 (Variables|/Game/RapidRideFightContent/Blueprints/CTF_GameModeBP.CTF_GameModeBP_C|GetRedFlag_Material _asctf_game_mode_bp)))
    (:NewEnumerator1
      (Rendering|Material|SetMaterial (Variables|Default|GetPickup) 0 (Variables|/Game/RapidRideFightContent/Blueprints/CTF_GameModeBP.CTF_GameModeBP_C|GetWhiteFlag_Material _asctf_game_mode_bp)))))