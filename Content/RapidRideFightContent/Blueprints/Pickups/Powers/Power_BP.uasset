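; Base-style power pickup Blueprint that gives its user a limited number of uses.
; On BeginPlay it binds to its use and use-finish events.
; Each use decrements the remaining count, with an in-use flag blocking further decrements until that use finishes.
; When a use finishes, it either clears the flag or, at zero uses, removes itself as the user's current pickup and destroys itself.
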(event Custom|Decrease%20Uses%20Left
  (params (User :type Boat%20BP%20Object%20Reference))
  (if (not (Variables|Default|GetInUse))
    (Variables|Default|SetInUse true)
    (Math|Integer|DecrementInt (Variables|Default|GetUsesLeft))))

(event Custom|CheckUsesLeft
  (if (== (Variables|Default|GetUsesLeft) 0)
    (Default|RemoveCurrentPickup (stale Custom|Decrease%20Uses%20Left User))
    (Actor|DestroyActor)
    (else
      (Variables|Default|SetInUse false))))

(event EventBeginPlay
  (EventDispatchers|BindEventtoOnUse (delegate Custom|Decrease%20Uses%20Left))
  (EventDispatchers|BindEventtoOnUseFinish (delegate Custom|CheckUsesLeft)))

(fn ConstructionScript)

(fn OnReponUse)