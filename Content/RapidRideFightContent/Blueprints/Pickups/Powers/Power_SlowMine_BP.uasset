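; Power_SlowMine_BP is a usable power pickup that drops a slow mine in the game world.
; On BeginPlay it binds DropMine to its parent's OnUse event.
; DropMine spawns a Pickup_SlowMine_BP at the user's Flag transform, passes it the user's team, then signals that use has finished.
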(event Custom|Drop%20Mine
  (params (User :type Boat%20BP%20Object%20Reference))
  (bind _returnvalue (Game|SpawnActorfromClass "/Game/RapidRideFightContent/Blueprints/Pickups/Pickup_SlowMine_BP.Pickup_SlowMine_BP_C" (Transformation|GetWorldTransform (Variables|/Game/RapidRideFightContent/Blueprints/Boat_BP.Boat_BP_C|GetFlag User)) "Undefined" 0 0))
  (Default|OnSpawn _returnvalue (Variables|/Game/RapidRideFightContent/Blueprints/Boat_BP.Boat_BP_C|GetTeam User))
  (Default|CallOnUseFinish))

(event EventBeginPlay
  (|CallParentFunction)
  (EventDispatchers|BindEventtoOnUse (delegate Custom|Drop%20Mine)))

(fn ConstructionScript
  (|CallParentFunction))