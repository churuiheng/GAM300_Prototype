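; Laser power pickup for boats, a weapon that damages opposing-team boats in a line ahead of the user.
; When used, it activates the user's laser particle effect and calls a server check, which waits briefly and calls the boat's missile handler.
; A forward multi box trace then applies laser damage to each enemy boat hit, with debug drawing left on, before signalling that use has finished.
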(event Custom|Fire%20Laser
  (params (User :type Boat%20BP%20Object%20Reference))
  (Components|Activation|Activate (Variables|/Game/RapidRideFightContent/Blueprints/Boat_BP.Boat_BP_C|GetPS_Laser User) false)
  (CallFunction|ServerLaserCheck User))

(event Custom|Server_LaserCheck
  (params (User :type Actor%20Object%20Reference))
  (bind _returnvalue (Transformation|GetActorLocation User))
  (Utilities|FlowControl|Delay 1.5)
  (bind _asboat_bp (Utilities|Casting|CastToBoat_BP User))
  (Default|HandleMissles _asboat_bp)
  (bind _outhits (Class|KismetSystemLibrary|BoxTraceMulti _returnvalue (+ _returnvalue (* (Transformation|GetActorForwardVector User) 7.9e+03)) "100.000000,100.000000,100.000000" (Transformation|GetActorRotation User) "TraceTypeQuery1" true (Utilities|Array|MakeArray User) "ForDuration" true))
  (for _array_element _outhits
    (bind _asboat_bp_2 (Utilities|Casting|CastToBoat_BP (.HitActor (Collision|BreakHitResult _array_element))))
    (if (Utilities|Enum|NotEqual(Enum) (Variables|/Game/RapidRideFightContent/Blueprints/Boat_BP.Boat_BP_C|GetTeam _asboat_bp_2) (Variables|/Game/RapidRideFightContent/Blueprints/Boat_BP.Boat_BP_C|GetTeam (stale Custom|Fire%20Laser User)))
      (Default|TakeDamage _asboat_bp_2 (Variables|Default|GetLaserDamage) _asboat_bp_2)))
  (Default|CallOnUseFinish))

(event EventBeginPlay
  (|CallParentFunction)
  (EventDispatchers|BindEventtoOnUse (delegate Custom|Fire%20Laser)))

(fn ConstructionScript
  (|CallParentFunction))