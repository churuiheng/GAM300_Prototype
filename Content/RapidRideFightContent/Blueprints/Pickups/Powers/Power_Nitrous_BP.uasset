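; Nitrous pickup power that refills the nitrous of the vehicle or character that uses it.
; On BeginPlay it binds AddNitro to the parent's OnUse event.
; AddNitro loops over the refill amount, raising the user's NitrousCount and NitrousAmount only while the count is below its maximum, then signals that use has finished.
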(event Custom|Add%20Nitro
  (params (User :type Boat%20BP%20Object%20Reference))
  (bind _nitrouscount (Variables|/Game/RapidRideFightContent/Blueprints/Boat_BP.Boat_BP_C|GetNitrousCount User))
  (for _index (range 0 (Variables|Default|GetAmountToRefill))
    (if (< _nitrouscount (Variables|/Game/RapidRideFightContent/Blueprints/Boat_BP.Boat_BP_C|GetMaxNitrousCount User))
      (Math|Integer|IncrementInt _nitrouscount
        (:%20%20
          (Math|Float|IncrementFloat (Variables|/Game/RapidRideFightContent/Blueprints/Boat_BP.Boat_BP_C|GetNitrousAmount User))))))
  (Default|CallOnUseFinish))

(event EventBeginPlay
  (|CallParentFunction)
  (EventDispatchers|BindEventtoOnUse (delegate Custom|Add%20Nitro)))

(fn ConstructionScript
  (|CallParentFunction))