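; Laser power-up pickup that kills enemy boats in a line ahead of the user.
; On BeginPlay it binds FireLaser to the OnUse event, which activates the user's laser particle system and waits briefly.
; It then box-traces forward from the user, with debug drawing left on, and reports each hit boat on an opposing team to CTF_GameModeBP as died.
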(event Custom|Fire%20Laser
  (params (User :type Boat%20BP%20Object%20Reference))
  (bind _returnvalue (Transformation|GetActorLocation User))
  (Components|Activation|Activate (Variables|/Game/RapidRideFightContent/Blueprints/Boat_BP.Boat_BP_C|GetPS_Laser User) false)
  (Utilities|FlowControl|Delay 1.5)
  (bind _outhits (Class|KismetSystemLibrary|BoxTraceMulti _returnvalue (+ _returnvalue (* (Transformation|GetActorForwardVector User) 4.9e+03)) "100.000000,100.000000,100.000000" (Transformation|GetActorRotation User) "TraceTypeQuery1" false (Utilities|Array|MakeArray User) "ForDuration" true))
  (for _array_element _outhits
    (bind _asboat_bp (Utilities|Casting|CastToBoat_BP (.HitActor (Collision|BreakHitResult _array_element))))
    (if (Utilities|Enum|NotEqual(Enum) (Variables|/Game/RapidRideFightContent/Blueprints/Boat_BP.Boat_BP_C|GetTeam _asboat_bp) (Variables|/Game/RapidRideFightContent/Blueprints/Boat_BP.Boat_BP_C|GetTeam User))
      (bind _asctf_game_mode_bp (Utilities|Casting|CastToCTF_GameModeBP (Game|GetGameMode)))
      (Default|CallOnPlayerDied _asctf_game_mode_bp _asboat_bp))))

(event EventBeginPlay
  (|CallParentFunction)
  (EventDispatchers|BindEventtoOnUse (delegate Custom|Fire%20Laser)))

(event Collision|EventActorBeginOverlap
  (params (OtherActor :type Actor%20Object%20Reference)))

(event EventTick
  (params (DeltaSeconds :type Float%20%28single-precision%29))
  (|CallParentFunction DeltaSeconds) ; This node is disabled and will not be called.\nDrag off pins to build functionality.
)

(fn ConstructionScript
  (|CallParentFunction))