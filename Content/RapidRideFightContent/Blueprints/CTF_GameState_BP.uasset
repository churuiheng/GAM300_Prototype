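; Game state for a capture-the-flag mode that runs the pre-game countdown and match timer and toggles the warm-up info text on the first player's top HUD.
; StartCountdown uses a FlipFlop to alternate between the short start countdown and the timed match.
; Tick uses a one-second Delay to decrement Minutes and Seconds, showing the countdown widget again for the match's last seconds.
; A Timeline pulses that widget's font size and opacity.
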(event Custom|StartCountdown
  ;[1 1 1] Set Timer
  (Variables|Default|SetStart%20Countdown true)
  (CallFunction|ShowGameStartCountDown)
  (Utilities|FlowControl|FlipFlop
    (:A
      (Variables|Default|SetMinutes 0)
      (Variables|Default|SetSeconds 5))
    (:B
      (Variables|Default|SetMinutes 5)
      (Variables|Default|SetSeconds 0)
      (Variables|Default|SetGameHasStarted true))))

(event Custom|StopCountdown
  ;[1 1 1] Set Timer
  (Variables|Default|SetStart%20Countdown false))

(event Custom|DisplayGameStartCountDown
  ;[1 1 1] Add CountDown Widget
  (bind _returnvalue (UserInterface|CreateWidget "/Game/RapidRideFightContent/Assets/UI/W_CountDown.W_CountDown_C"))
  (bind _output_get (Variables|Default|SetGameStartWidget _returnvalue))
  (UserInterface|Viewport|AddtoViewport _output_get 0))

(event Custom|HideGameStartCountDown
  ;[1 1 1] Hide CountDown
  (Widget|SetVisibility (Variables|Default|GetGameStartWidget) "Hidden"))

(event Custom|ShowGameStartCountDown
  ;[1 1 1] Show CountDown
  (Widget|SetVisibility (Variables|Default|GetGameStartWidget) "Visible"))

(event Custom|Rescale
  (bind _gamestartwidget (Variables|Default|GetGameStartWidget))
  ;[1 1 1] AnimateCountDown
  (bind (_direction _fontsize _opacity) (Timeline|ChangeFontSize PlayFromStart)
    (:Update
      (Variables|/Game/RapidRideFightContent/Assets/UI/W_CountDown.W_CountDown_C|SetFontSize _gamestartwidget (Math|Float|Truncate (Math|Float|Lerp 144.0 2e+02 _fontsize)))
      (Variables|/Game/RapidRideFightContent/Assets/UI/W_CountDown.W_CountDown_C|SetOpacity _gamestartwidget (Math|Float|Lerp 0.0 1.0 _opacity)))
    (:Finished
      (if (== (Variables|Default|GetSeconds) 0)
        (Utilities|FlowControl|DoOnce false
          (:Completed
            (CallFunction|Rescale)
            (Development|PrintString "Hello")))
        (else
          (CallFunction|Rescale))))))

(event Custom|AnimateCountDown
  (bind _gamestartwidget (Variables|Default|GetGameStartWidget))
  ;[1 1 1] AnimateCountDown
  (bind (_direction _fontsize _opacity) (Timeline|ChangeFontSize Play)
    (:Update
      (Variables|/Game/RapidRideFightContent/Assets/UI/W_CountDown.W_CountDown_C|SetFontSize _gamestartwidget (Math|Float|Truncate (Math|Float|Lerp 144.0 2e+02 _fontsize)))
      (Variables|/Game/RapidRideFightContent/Assets/UI/W_CountDown.W_CountDown_C|SetOpacity _gamestartwidget (Math|Float|Lerp 0.0 1.0 _opacity)))
    (:Finished
      (if (== (Variables|Default|GetSeconds) 0)
        (Utilities|FlowControl|DoOnce false
          (:Completed
            (CallFunction|Rescale)
            (Development|PrintString "Hello")))
        (else
          (CallFunction|Rescale))))))

(event Custom|ShowEndCountDownText
  ;[1 1 1] AnimateCountDown
  (Utilities|FlowControl|DoOnce false) ; enters at Reset
)

(event Custom|HideInfoText
  ;[1 1 1] HideInfoText (WarmUp)
  (bind _tophud (Class|BoatControllerBPI|GetTopHUD(Message) (Game|GetPlayerController 0)))
  (Default|HideInfoText _tophud))

(event Custom|DisplayInfoText
  ;[1 1 1] DisplayInfoText
  (bind _tophud (Class|BoatControllerBPI|GetTopHUD(Message) (Game|GetPlayerController 0)))
  (Default|ShowInfoText _tophud))

(event EventBeginPlay
  (CallFunction|DisplayGameStartCountDown)
  (if (Variables|Default|GetStart%20Countdown)
    (CallFunction|ShowGameStartCountDown)
    (else
      (CallFunction|HideGameStartCountDown))))

(event EventTick
  (params (DeltaSeconds :type Float%20%28single-precision%29))
  (bind _minutes (Variables|Default|GetMinutes))
  (if (Variables|Default|GetStart%20Countdown)
    (CallFunction|AnimateCountDown)
    (Utilities|FlowControl|Delay 1.0)
    (CallFunction|ShowEndCountDownText)
    (if (== (Variables|Default|GetSeconds) 0)
      (if (== _minutes 0)
        (if (Variables|Default|GetGameHasStarted)
          ;[1 1 1] If countdown end...
          (Variables|Default|SetLastFewSeconds false)
          (Variables|Default|SetStart%20Countdown false)
          (Variables|Default|SetGameHasStarted false)
          (CallFunction|HideGameStartCountDown)
          (CallFunction|DisplayInfoText)
          (else
            ;[1 1 1] Game Start countdown end... Games Begin
            (CallFunction|StartCountdown)
            (CallFunction|HideGameStartCountDown)
            (CallFunction|HideInfoText)))
        (else
          (Math|Integer|DecrementInt _minutes
            (:%20%20
              (Variables|Default|SetSeconds 59)))))
      (else
        (Math|Integer|DecrementInt (Variables|Default|GetSeconds)
          (:%20%20
            (if (Variables|Default|GetGameHasStarted)
              (if (and (== (Variables|Default|GetMinutes) 0) (<= (Variables|Default|GetSeconds) 3))
                (Variables|Default|SetLastFewSeconds true)
                (CallFunction|ShowGameStartCountDown)
                (else
                  (Variables|Default|SetLastFewSeconds false)
                  (CallFunction|HideGameStartCountDown))))))))))

(fn ConstructionScript)