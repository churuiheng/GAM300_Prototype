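; Player-controlled jet boat pawn for a team capture-the-flag mode, with an orbit camera.
; Input drives physics forces and yaw, while Tick applies side drag against sliding and extra turn while drifting.
; Limited nitrous boosts add an impulse with FOV, shake and rumble effects.
; Keys pick team and hull material; a looping timer refreshes flag bases via client-to-server events, and carrying the flag scales movement force.
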(event Custom|Client_AssignTeam
  (params (Team :type Team_Enum%20Enum :default "NewEnumerator0"))
  ;[0.8436 0.2258 0.7316 1 48] CAPTURE THE FLAG STUFF
  ;;[0.1038 0.1038 0.1038] Assign Team
  (CallFunction|ServerAssignTeam Team)
  (CallFunction|ClientCreateHUD))

(event Custom|Server_AssignTeam
  (params (Team :type Team_Enum%20Enum :default "NewEnumerator0"))
  ;[0.8436 0.2258 0.7316 1 48] CAPTURE THE FLAG STUFF
  ;;[0.1038 0.1038 0.1038] Assign Team
  (Variables|In-GameVariables|SetTeam Team))

(event Custom|Client_CreateHUD
  ;[0.8436 0.2258 0.7316 1 48] CAPTURE THE FLAG STUFF
  ;;[0.1038 0.1038 0.1038] Create HUD
  (bind _returnvalue (UserInterface|CreateWidget "/Game/RapidRideFightContent/Widgets_UI/W_TopHUD.W_TopHUD_C" (Game|GetPlayerController 0) self))
  (UserInterface|Viewport|AddtoViewport _returnvalue 0))

(event Custom|UpdateInfo
  ;[0.8436 0.2258 0.7316 1 48] CAPTURE THE FLAG STUFF
  ;;[0.1038 0.1038 0.1038] Network Update Info
  (CallFunction|ClientUpdateInfo (Variables|In-GameVariables|GetTeam)))

(event Custom|Server_UpdateInfo
  (params (Team :type Team_Enum%20Enum :default "NewEnumerator0"))
  ;[0.8436 0.2258 0.7316 1 48] CAPTURE THE FLAG STUFF
  ;;[0.1038 0.1038 0.1038] Network Update Info
  (bind _outactors (Actor|GetAllActorsOfClass "/Game/RapidRideFightContent/Blueprints/FlagBase/FlagBase_BP.FlagBase_BP_C"))
  (bind _array_element (Utilities|Array|ForEachLoopwithBreak _outactors)
    (:LoopBody
      (if (Utilities|Enum|Equal(Enum) (Variables|/Game/RapidRideFightContent/Blueprints/FlagBase/FlagBase_BP.FlagBase_BP_C|GetTeam _array_element) Team)
        (Variables|In-GameVariables|SetMyFlagBase _array_element)
        (else
          (Variables|In-GameVariables|SetEnemyFlagBase _array_element))))))

(event Custom|Client_UpdateInfo
  (params (Team :type Team_Enum%20Enum :default "NewEnumerator0"))
  ;[0.8436 0.2258 0.7316 1 48] CAPTURE THE FLAG STUFF
  ;;[0.1038 0.1038 0.1038] Network Update Info
  (CallFunction|ServerUpdateInfo Team))

(event EventBeginPlay
  ;[0.8436 0.2258 0.7316 1 48] CAPTURE THE FLAG STUFF
  ;;[0.1038 0.1038 0.1038] Network Update Info
  (Utilities|Time|SetTimerbyEvent (delegate Custom|UpdateInfo) 0.25 true))

(event EventTick
  (params (DeltaSeconds :type Float%20%28single-precision%29))
  (bind _returnvalue (Transformation|GetActorRightVector))
  (bind _boat (Variables|Default|GetBoat))
  (bind _boat_2 (Variables|Default|GetBoat))
  (bind _returnvalue_2 (Transformation|GetComponentVelocity _boat_2))
  (bind _returnvalue_3 (Math|Vector|Normalize _returnvalue_2))
  ;[1 1 1] Movement
  (Utilities|FlowControl|Sequence
    (:then_0
      (if (or (!= (Input|AxisValues|GetMoveRight) 0.0) (> (Input|AxisValues|GetMoveForward) 0.0))
        (Variables|In-GameVariables|SetisMoving true)
        (else
          (Variables|In-GameVariables|SetisMoving false))))
    (:then_1
      ;;[1 1 1] Turn sharper, increase side drag
      (if (not (< (Math|Float|Absolute(Float) (- (.X (Math|Vector|BreakVector (Math|Rotator|GetRotationXVector (Transformation|GetWorldRotation _boat_2)))) (.X (Math|Vector|BreakVector (Math|Rotator|GetRotationXVector (Math|Conversions|RotationFromXVector _returnvalue_3)))))) (Variables|Parameters|GetSlipperyFactor)))
        (Physics|AddForce _boat (* _returnvalue (* -1 (* (Variables|Parameters|GetHandlingAmount) (* (Math|Float|Sign(Float) (Math|Vector|DotProduct _returnvalue_3 _returnvalue)) (Math|Vector|VectorLength (Transformation|GetComponentVelocity _boat)))))) "None" false)))
    (:then_2
      (CallFunction|Drift DeltaSeconds))))

(event Input|ActionEvents|InputActionDrift
  (params (Key :type Key%20Structure :default "None"))
  ;[1 1 1] Input Actions
  (:Pressed
    (if (Variables|In-GameVariables|GetcanDrift)
      (Variables|In-GameVariables|SetisDrifting true)
      (bind _returnvalue (Physics|GetPhysicsLinearVelocity (Variables|Default|GetBoat) "None"))
      (Variables|In-GameVariables|SetspeedBeforeDrift (Math|Vector|VectorLength _returnvalue))
      (else
        (Variables|In-GameVariables|SetisDrifting false))))
  (:Released
    (Variables|In-GameVariables|SetisDrifting false)
    (Variables|In-GameVariables|SetcanDrift true)))

(event Input|ActionEvents|InputActionBoost
  (params (Key :type Key%20Structure :default "None"))
  (bind _boat (Variables|Default|GetBoat))
  (bind _nitrouscount (Variables|In-GameVariables|GetNitrousCount))
  ;[1 1 1] Input Actions
  (:Pressed
    (if (and (Variables|In-GameVariables|GetcanBoost) (> _nitrouscount 0))
      (Math|Integer|DecrementInt _nitrouscount
        (:%20%20
          (Variables|In-GameVariables|SetcanBoost false)
          (Physics|AddImpulse _boat (* (Math|Vector|GetForwardVector (Variables|Default|GetBoat)) (Variables|Parameters|GetBoosterAmount)) "None" true)
          (Physics|AddImpulseatLocation _boat "0.000000,0.000000,-10000.000000" (Transformation|GetWorldLocation (Variables|Default|GetBoostEffectLocation)) "None")
          (Camera|PlayWorldCameraShake "/Game/RapidRideFightContent/Blueprints/CameraShake/CameraShake_Boost.CameraShake_Boost_C" (Transformation|GetWorldLocation (Variables|Default|GetCamera)) 0.0 1e+02)
          (Game|Feedback|ClientPlayForceFeedback (Game|GetPlayerController 0) "/Game/RapidRideFightContent/ControllerFeedback/ControllerFeedback_Boost.ControllerFeedback_Boost" "None" false false false)
          (Utilities|FlowControl|Sequence
            (:then_0
              (bind _fov (Timeline|FieldOfView PlayFromStart)
                (:Update
                  (Camera|SetFieldOfView (Variables|Default|GetCamera) _fov))
                (:Finished
                  (Variables|In-GameVariables|SetcanBoost true)
                  (Timeline|FieldOfView SetNewTime))))
            (:then_1
              (bind _deltatime (Timeline|LerpNitrous PlayFromStart)
                (:Update
                  (Variables|In-GameVariables|SetNitrousAmount (+ _deltatime (Math|Conversions|ToFloat(Integer) (Variables|In-GameVariables|GetNitrousCount)))))))))))))

(event Input|AxisEvents|InputAxisMoveForward
  (params (AxisValue :type Float%20%28single-precision%29))
  ;[1 1 1] Movement
  (bind _returnvalue (Physics|GetPhysicsLinearVelocity (Variables|Default|GetBoat) "None"))
  (if (< (Math|Vector|VectorLength _returnvalue) (Variables|In-GameVariables|GetcurrentMaxSpeed))
    _
    (else
      _))
  (Physics|AddForce (Variables|Default|GetBoat) (* (Transformation|GetActorForwardVector) (* AxisValue (* (Variables|In-GameVariables|GetcurrentMovementSpeed) 1e+02))) "None" false)
  (Effects|SpawnEmitterAttached 0 (Variables|Default|GetSplashEmitter) "None" "0, 0, 0" "0, 0, 0" "1.000000,1.000000,1.000000" "KeepRelativeOffset" true "None" (Variables|In-GameVariables|GetisMoving)))

(event Input|AxisEvents|InputAxisMoveRight
  (params (AxisValue :type Float%20%28single-precision%29))
  (bind _boat (Variables|Default|GetBoat))
  ;[1 1 1] Movement
  (Transformation|AddRelativeRotation _boat (Math|Rotator|MakeRotator 0.0 0.0 (* AxisValue (Variables|Parameters|GetRotationSpeed))) false false)
  (Physics|AddForce (Variables|Default|GetBoat) (* (Transformation|GetActorRightVector) (* 1e+01 (Math|Vector|VectorLength (Transformation|GetComponentVelocity _boat)))) "None" false)
  (Effects|SpawnEmitterAttached 0 (Variables|Default|GetSplashEmitter) "None" "0, 0, 0" "0, 0, 0" "1.000000,1.000000,1.000000" "KeepRelativeOffset" true "None" (Variables|In-GameVariables|GetisMoving)))

(event Input|AxisEvents|InputAxisLookUp
  (params (AxisValue :type Float%20%28single-precision%29))
  ;[1 1 1] Mouse Control
)

(event Input|AxisEvents|InputAxisTurn
  (params (AxisValue :type Float%20%28single-precision%29))
  ;[1 1 1] Mouse Control
)

(event Input|AxisEvents|InputAxisLookUpRate
  (params (AxisValue :type Float%20%28single-precision%29))
  ;[1 1 1] Mouse Control
  (Transformation|AddRelativeRotation (Variables|Default|GetSpringArm) (Math|Rotator|MakeRotator 0.0 AxisValue 0.0) false false))

(event Input|AxisEvents|InputAxisTurnRate
  (params (AxisValue :type Float%20%28single-precision%29))
  ;[1 1 1] Mouse Control
  (Transformation|AddRelativeRotation (Variables|Default|GetSpringArm) (Math|Rotator|MakeRotator 0.0 0.0 AxisValue) false false))

(event Input|KeyboardEvents|1
  (params (Key :type Key%20Structure :default "None"))
  ;[0.8436 0.2258 0.7316 1 48] CAPTURE THE FLAG STUFF
  ;;[0.1038 0.1038 0.1038] Assign Team
  (:Pressed
    (CallFunction|ClientAssignTeam "NewEnumerator0")
    (Rendering|Material|SetMaterial (Variables|Default|GetBoat) 0 "/Game/RapidRideFightContent/Assets/MATERIALS/M_JetBoat_R3B.M_JetBoat_R3B")
    (Rendering|Material|SetMaterial (Variables|Default|GetFlag) 0 0)))

(event Input|GamepadEvents|GamepadLeftShoulder
  (params (Key :type Key%20Structure :default "None"))
  ;[0.8436 0.2258 0.7316 1 48] CAPTURE THE FLAG STUFF
  ;;[0.1038 0.1038 0.1038] Assign Team
  (:Pressed
    (CallFunction|ClientAssignTeam "NewEnumerator1")
    (Rendering|Material|SetMaterial (Variables|Default|GetBoat) 0 "/Game/RapidRideFightContent/Assets/MATERIALS/M_JetBoat_W3B.M_JetBoat_W3B")
    (Rendering|Material|SetMaterial (Variables|Default|GetFlag) 0 0)))

(event Input|KeyboardEvents|2
  (params (Key :type Key%20Structure :default "None"))
  ;[0.8436 0.2258 0.7316 1 48] CAPTURE THE FLAG STUFF
  ;;[0.1038 0.1038 0.1038] Assign Team
  (:Pressed
    (CallFunction|ClientAssignTeam "NewEnumerator1")
    (Rendering|Material|SetMaterial (Variables|Default|GetBoat) 0 "/Game/RapidRideFightContent/Assets/MATERIALS/M_JetBoat_W3B.M_JetBoat_W3B")
    (Rendering|Material|SetMaterial (Variables|Default|GetFlag) 0 0)))

(event Input|GamepadEvents|GamepadRightShoulder
  (params (Key :type Key%20Structure :default "None"))
  ;[0.8436 0.2258 0.7316 1 48] CAPTURE THE FLAG STUFF
  ;;[0.1038 0.1038 0.1038] Assign Team
  (:Pressed
    (CallFunction|ClientAssignTeam "NewEnumerator0")
    (Rendering|Material|SetMaterial (Variables|Default|GetBoat) 0 "/Game/RapidRideFightContent/Assets/MATERIALS/M_JetBoat_R3B.M_JetBoat_R3B")
    (Rendering|Material|SetMaterial (Variables|Default|GetFlag) 0 0)))

(fn ConstructionScript)

(fn Drift
  (params (Ticks :type Float%20%28single-precision%29))
  (if (Variables|In-GameVariables|GetisDrifting)
    (if (< (Variables|Parameters|GetDriftAmount) (Variables|Parameters|GetMaxDriftAmount))
      (if (!= (Input|AxisValues|GetMoveRight) 0.0)
        (Transformation|AddRelativeRotation (Variables|Default|GetBoat) (Math|Rotator|MakeRotator 0.0 0.0 (* (+ (Input|AxisValues|GetMoveForward) 1.0) (* (Variables|Parameters|GetDriftAmount) (Input|AxisValues|GetMoveRight)))) false false)
        (bind _returnvalue (Physics|GetPhysicsLinearVelocity (Variables|Default|GetBoat) "None"))
        ;[1 1 1] Reduce slip if forward pressed and current speed less than before drift
        (if (and (< (Math|Vector|VectorLength _returnvalue) (Variables|In-GameVariables|GetspeedBeforeDrift)) (!= (Input|AxisValues|GetMoveForward) 0.0))
          (Physics|AddForce (Variables|Default|GetBoat) (* (Transformation|GetActorRightVector) (* (Input|AxisValues|GetMoveRight) (Variables|In-GameVariables|GetcurrentMovementSpeed))) "None" true)))
      (else
        (Variables|In-GameVariables|SetcanDrift false)))
    (elif (> (Variables|Parameters|GetDriftAmount) 1.0)
      (Variables|Parameters|SetDriftAmount 1.0))))

(fn OnFlagPickup
  (Rendering|SetVisibility (Variables|Default|GetFlag) true false)
  (Variables|In-GameVariables|SetcurrentMovementSpeed (* (Variables|Parameters|GetSpeedRatio_WithFlag) (Variables|Parameters|GetMovementSpeed)))
  (Variables|In-GameVariables|SetisCarryingFlag true))

(fn OnFlagRemove
  (Rendering|SetVisibility (Variables|Default|GetFlag) false false)
  (Variables|In-GameVariables|SetcurrentMovementSpeed (Variables|Parameters|GetMovementSpeed))
  (Variables|In-GameVariables|SetisCarryingFlag false))