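; BoatBP is a player-controlled boat that moves by physics forces, scaled by BoosterAmount, with steering adding both yaw and sideways force.
; Both movement axes spawn a poof emitter on every event, auto-activated by an IsMoving flag that Tick sets from input.
; Tick's auto-adjust yaw math is multiplied by zero, so it has no effect.
; K destroys the boat; mouse look, velocity-facing and spawn-location saving are unwired.
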(event EventBeginPlay)

(event EventTick
  (params (DeltaSeconds :type Float%20%28single-precision%29))
  (bind _returnvalue (Pawn|GetControlRotation :!class /Script/Engine.Pawn))
  (bind _returnvalue_2 (Input|AxisValues|GetMoveRight))
  (bind _returnvalue_3 (Input|AxisValues|GetMoveForward))
  (bind _yaw (Math|Rotator|BreakRotator _returnvalue))
  (bind _returnvalue_4 (Math|Rotator|MakeRotator 0.0 0.0 _yaw))
  (bind _returnvalue_5 (Math|Vector|GetForwardVector _returnvalue_4))
  (bind _returnvalue_6 (Math|Vector|GetRightVector _returnvalue_4))
  (bind _returnvalue_7 (* _returnvalue_5 _returnvalue_3))
  (bind _returnvalue_8 (* _returnvalue_6 _returnvalue_2))
  (bind _returnvalue_9 (+ _returnvalue_7 _returnvalue_8))
  (bind _returnvalue_10 (Math|Vector|Normalize _returnvalue_9))
  (Utilities|FlowControl|Sequence
    (:then_0
      (if (or (!= (Input|AxisValues|GetMoveRight) 0.0) (> (Input|AxisValues|GetMoveForward) 0.0))
        (Variables|Default|SetisMoving true)
        (else
          (Variables|Default|SetisMoving false))))
    (:then_1
      ;[1 1 1] Camera Auto Adjustment
      (Transformation|AddRelativeRotation (Variables|Default|GetBoat) (Math|Rotator|MakeRotator 0.0 0.0 (* (Math|Float|Clamp(Float) (* 0.0 (Math|Float|Clamp(Float) (+ (Math|Float|Absolute(Float) (Input|AxisValues|GetMoveForward)) (Math|Float|Absolute(Float) (Input|AxisValues|GetMoveRight)))) (Math|Float|Power (- 1.0 (Math|Float|Absolute(Float) (Math|Vector|DotProduct (Math|Vector|GetForwardVector (Math|Rotator|MakeRotator 0.0 0.0 (.Yaw (Math|Rotator|BreakRotator (Pawn|GetControlRotation :!class /Script/Engine.Pawn))))) _returnvalue_10))) (Variables|Default|GetAngleExponent)) (Variables|Default|GetCameraComponentRate))) (.Yaw (Math|Rotator|BreakRotator (Math|Rotator|Delta(Rotator) (Math|Conversions|RotationFromXVector _returnvalue_10) (Pawn|GetControlRotation :!class /Script/Engine.Pawn)))))) false false))))

(event Input|AxisEvents|InputAxisMoveForward
  (params (AxisValue :type Float%20%28single-precision%29))
  ;[1 1 1] Movement
  (Physics|AddForce (Variables|Default|GetBoat) (* (Transformation|GetActorForwardVector) (* (* -1 (* AxisValue 1e+05)) (Variables|Default|GetBoosterAmount))) "None" false)
  (Effects|SpawnEmitterAttached "/Game/RapidRideFightContent/Assets/Poof/PS_Poof.PS_Poof" (Variables|Default|GetSplashEmitter) "None" "0, 0, 0" "0, 0, 0" "1.000000,1.000000,1.000000" "KeepRelativeOffset" true "None" (Variables|Default|GetisMoving)))

(event Input|AxisEvents|InputAxisMoveRight
  (params (AxisValue :type Float%20%28single-precision%29))
  ;[1 1 1] Movement
  (Transformation|AddRelativeRotation (Variables|Default|GetBoat) (Math|Rotator|MakeRotator 0.0 0.0 (* AxisValue (Variables|Default|GetRotationSpeed))) false false)
  (Physics|AddForce (Variables|Default|GetBoat) (* (Transformation|GetActorRightVector) (* (* -1 (* AxisValue 8e+04)) (Variables|Default|GetBoosterAmount))) "None" false)
  (Effects|SpawnEmitterAttached "/Game/RapidRideFightContent/Assets/Poof/PS_Poof.PS_Poof" (Variables|Default|GetSplashEmitter) "None" "0, 0, 0" "0, 0, 0" "1.000000,1.000000,1.000000" "KeepRelativeOffset" true "None" (Variables|Default|GetisMoving)))

(event Input|AxisEvents|InputAxisLookUp
  (params (AxisValue :type Float%20%28single-precision%29))
  ;[1 1 1] Mouse Control
)

(event Input|AxisEvents|InputAxisTurn
  (params (AxisValue :type Float%20%28single-precision%29))
  ;[1 1 1] Mouse Control
)

(event Input|KeyboardEvents|K
  (params (Key :type Key%20Structure :default "None"))
  (:Pressed
    (Actor|DestroyActor)))

(fn ConstructionScript)